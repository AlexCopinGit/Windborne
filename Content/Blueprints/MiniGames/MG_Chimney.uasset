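; Chimney valve minigame, started with Interact at the chimney when it needs attention, that locks player input and focuses the camera.
; A deprojected mouse hand sprite drags the valve: turns matching a periodically randomized arrow raise the gauge, wrong turns and time lower it.
; Holding the gauge in a target band for a set time wins and notifies MG_Manager.
; DifficultySteps tunes turn threshold, decay and hold time.
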(event `ClickEvent`
  (bind _valvespeed (`self.ValveSpeed`))
  (bind (_returnvalue_x _returnvalue_y _returnvalue_z) (`KismetMathLibrary.BreakVector` (`SceneComponent.K2_GetComponentLocation` (`self.Valve`))))
  (bind _worldlocation (`PlayerController.DeprojectMousePositionToWorld` (`GameplayStatics.GetPlayerController` 0)))
  (bind _returnvalue (`KismetMathLibrary.FClamp` (- (`self.MousePosBefore`) (.x _worldlocation)) (* _valvespeed -1.0) _valvespeed))
  ;[1 1 1] ClickEvent
  (if (`PrimitiveComponent.IsOverlappingComponent` (`self.Valve`) (`self.Mouse`))
    (if (`self.LeftClickPressed`)
      (`|ExecutionSequence`
        (:`then_0`
          (if (< (.z _worldlocation) _returnvalue_z)
            (set `self.SpeedRotation` (* _returnvalue -1.0))
            (else
              (set `self.SpeedRotation` _returnvalue)))
          (`SceneComponent.K2_AddWorldRotation` (`self.Valve`) (`KismetMathLibrary.MakeRotator` 0.0 (`self.SpeedRotation`)) false false)
          (set `self.MousePosBefore` (.x (`PlayerController.DeprojectMousePositionToWorld` (`GameplayStatics.GetPlayerController` 0)))))
        (:`then_1`
          (if (> (`self.SpeedRotation`) 0.0)
            (set `self.TurningLeft` true)
            (set `self.TurningRight` false)
            (elif (< (`self.SpeedRotation`) 0.0)
              (set `self.TurningLeft` false)
              (set `self.TurningRight` true))))))))

(event `self.ReceiveBeginPlay`
  ;[1 1 1] BeginPlay
  (`|ExecutionSequence`
    (:`then_0`
      (bind _outactors (`GameplayStatics.GetAllActorsOfClass` "/Game/Blueprints/Char.Char_C"))
      (set `self.Player` (`|GetArrayItem` _outactors)))
    (:`then_1`
      (bind _outactors_2 (`GameplayStatics.GetAllActorsOfClass` "/Game/Blueprints/Cam.Cam_C"))
      (set `self.Cam` (`|GetArrayItem` _outactors_2)))
    (:`then_2`
      (bind _ashud_main (cast `/Game/UI/HUD_Main` (`PlayerController.GetHUD` (`GameplayStatics.GetPlayerController` 0))))
      (set `self.HUD` _ashud_main)
      (`self.ActivateDeactivateMouseAndValve` false)
      (set `self.TimeToWin` (`self.TimeToWinValue`)))
    (:`then_3`
      (bind _outactors_3 (`GameplayStatics.GetAllActorsOfClass` "/Game/Blueprints/Ship.Ship_C"))
      (set `self.Ship` (`|GetArrayItem` _outactors_3)))
    (:`then_4`
      (set `self.LocOffset` (`self.K2_GetActorLocation`)))
    (:`then_5`
      (bind _outactors_4 (`GameplayStatics.GetAllActorsOfClass` "/Game/Blueprints/MiniGames/MG_Manager.MG_Manager_C"))
      (set `self.MGManager` (`|GetArrayItem` _outactors_4))
      (set `self.LastSprite` "/Game/Sprites/MiniGames/ChimneyGauge/Chimney_Gauge_Sprite_0.Chimney_Gauge_Sprite_0")
      (`self.DisplaySpritesMG` true)
      (`SceneComponent.K2_SetRelativeLocation` (`self.Valve`) (0.0 21.0 48.0) false false))))

(event `self.ReceiveTick`
  (params (DeltaSeconds :type "Float (single-precision)"))
  (bind _worldlocation (`PlayerController.DeprojectMousePositionToWorld` (`GameplayStatics.GetPlayerController` 0)))
  ;[1 1 1] Tick
  (set `self.DeltaTime` DeltaSeconds)
  (`|ExecutionSequence`
    (:`then_0`
      (if (`self.NeedPlayerAction`)
        (set `self.IsPlaying` true)
        (if (not (`self.CanPlayerInteract`))
          (`self.ChangeSprites` false true))
        (else
          (`self.ChangeSprites` false))))
    (:`then_1`
      (if (`self.IsActive`)
        _))
    (:`then_2`
      (`SceneComponent.K2_SetWorldLocation` (`self.Mouse`) (`KismetMathLibrary.MakeVector` (.x _worldlocation) 25.0 (.z _worldlocation)) false false))
    (:`then_3`
      (if (`self.IsActive`)
        (`|ExecutionSequence`
          (:`then_0`
            (`self.ClickEvent`))
          (:`then_1`
            (`self.GameplayLoop`)))))))

(event `ChangeSprites`
  (params (Interact :type Boolean) (MGNeedPlayer :type Boolean))
  ;[1 1 1] ChangeSprites
  (if Interact
    (`PaperFlipbookComponent.SetFlipbook` (`self.ChimneyFlip`) "/Game/Anim/MiniGames/ChimneyInteract.ChimneyInteract")
    (`PaperFlipbookComponent.SetFlipbook` (`self.ValveFlip`) "/Game/Anim/MiniGames/ChimneyInteract2.ChimneyInteract2")
    (elif MGNeedPlayer
      (`PaperFlipbookComponent.SetFlipbook` (`self.ChimneyFlip`) "/Game/Anim/MiniGames/ChimneyActive.ChimneyActive")
      (`PaperFlipbookComponent.SetFlipbook` (`self.ValveFlip`) "/Game/Anim/MiniGames/ChimneyActive2.ChimneyActive2")
      (else
        (`PaperFlipbookComponent.SetFlipbook` (`self.ChimneyFlip`) "/Game/Anim/MiniGames/ChimneyIdle.ChimneyIdle")
        (`PaperFlipbookComponent.SetFlipbook` (`self.ValveFlip`) "/Game/Anim/MiniGames/ChimneyIdle2.ChimneyIdle2")))))

(event `self.ReceiveActorBeginOverlap`
  (params (OtherActor :type "Actor Object Reference"))
  ;[1 1 1] Overlap
  (if (`self.NeedPlayerAction`)
    (set `self.CanPlayerInteract` true)
    (`self.ChangeSprites` true)))

(event `GameplayLoop`
  (bind _steppassed (`self.StepPassed`))
  (bind _volumemultiplier (`/Game/Blueprints/Ship.VolumeMultiplier` (`self.Ship`)))
  (bind _returnvalue (`KismetMathLibrary.Clamp` (- (`self.StepPassed`) 1) 0 22))
  (`|ExecutionSequence`
    (:`then_0`
      (set `self.Rotation` (+ (`self.Rotation`) (`self.SpeedRotation`)))
      (if (and (`self.HaveToTurnLeft`) (`self.TurningLeft`) (>= (`self.Rotation`) (`self.RotationValueToReach`)))
        (set `self.StepPassed` (`KismetMathLibrary.Clamp` (+ (`self.StepPassed`) 1) 0 22))
        (set `self.Rotation` 0.0)
        (`GameplayStatics.PlaySound2D` (`self.TurnValveSound`) (`/Game/Blueprints/Ship.VolumeMultiplier` (`self.Ship`)) 1.0 0.0 null null)
        (elif (and (`self.HaveToTurnRight`) (<= (`self.Rotation`) (* (`self.RotationValueToReach`) -1.0)) (`self.TurningRight`))
          (set `self.StepPassed` (`KismetMathLibrary.Clamp` (+ (`self.StepPassed`) 1) 0 22))
          (set `self.Rotation` 0.0)
          (`GameplayStatics.PlaySound2D` (`self.TurnValveSound`) (`/Game/Blueprints/Ship.VolumeMultiplier` (`self.Ship`)) 1.0 0.0 null null)
          (elif (and (not (`self.HaveToTurnRight`)) (<= (`self.Rotation`) (* (`self.RotationValueToReach`) -1.0)) (`self.TurningRight`))
            (set `self.StepPassed` _returnvalue)
            (set `self.Rotation` 0.0)
            (`GameplayStatics.PlaySound2D` (`self.TurnValveSound`) _volumemultiplier 1.0 0.0 null null)
            (elif (and (not (`self.HaveToTurnLeft`)) (>= (`self.Rotation`) (`self.RotationValueToReach`)) (`self.TurningLeft`))
              (set `self.StepPassed` _returnvalue)
              (set `self.Rotation` 0.0)
              (`GameplayStatics.PlaySound2D` (`self.TurnValveSound`) _volumemultiplier 1.0 0.0 null null))))))
    (:`then_1`
      (`KismetSystemLibrary.Delay` (`self.CooldownLoseStep`))
      (set `self.StepPassed` (`KismetMathLibrary.Clamp` (- (`self.StepPassed`) 1) 0 22)))
    (:`then_2`
      (`PaperSpriteComponent.SetSprite` (`self.Chimney_Gauge`) (`|GetArrayItem` (`self.ChimneyGauges`) (`self.StepPassed`)))
      (if (and (> _steppassed 15) (< _steppassed 19))
        (bind _output_get (set `self.TimeToWin` (- (`self.TimeToWin`) (`self.DeltaTime`))))
        (if (<= _output_get 0.0)
          (`self.WinGame`))
        (else
          (set `self.TimeToWin` (`KismetMathLibrary.FClamp` (+ (`self.TimeToWin`) (`self.DeltaTime`)) 0.0 (`self.TimeToWinValue`))))))
    (:`then_3`
      (`KismetSystemLibrary.Delay` 5.0)
      (if (`self.IsActive`)
        (`self.ChangeSideToTurn`)))))

(event `self.ReceiveActorEndOverlap`
  (params (OtherActor :type "Actor Object Reference"))
  ;[1 1 1] Overlap
  (if (`self.NeedPlayerAction`)
    (set `self.CanPlayerInteract` false)))

(event `MG_Start`
  (bind _hud (`self.HUD`))
  (bind _player (`self.Player`))
  (bind (_returnvalue_x _returnvalue_y _returnvalue_z) (`KismetMathLibrary.BreakVector` (`self.K2_GetActorLocation` _player)))
  (bind (_returnvalue_x_2 _returnvalue_y_2 _returnvalue_z_2) (`KismetMathLibrary.BreakVector` (`self.K2_GetActorLocation` _player)))
  (bind _boxextent_x (`KismetMathLibrary.BreakVector` (`BoxComponent.BoxExtent` (`self.Box`))))
  (bind _boxextent_x_2 (`KismetMathLibrary.BreakVector` (`BoxComponent.BoxExtent` (`self.Box`))))
  ;[1 1 1] StartGame
  (set `self.IsActive` true)
  (`self.DisableInput` (`self.Player`) null)
  (`self.DisplaySpritesMG` false)
  (if (`/Game/Blueprints/Char.IsFlipped` _player)
    (`self.K2_SetActorLocation` _player (`KismetMathLibrary.MakeVector` (* 3 _boxextent_x) _returnvalue_y_2 _returnvalue_z_2) false false)
    (else
      (`self.K2_SetActorLocation` _player (`KismetMathLibrary.MakeVector` (* -1 _boxextent_x_2) _returnvalue_y _returnvalue_z) false false)))
  (`/Game/Blueprints/Cam.FocusMG` (`self.Cam`) true (`self.LocOffset`))
  (`/Game/UI/HUD_Main.ShowWidgets` _hud false)
  (`/Game/UI/HUD_Main.CenterCursor` _hud)
  (`self.ActivateDeactivateMouseAndValve` true)
  (`self.ChangeSideToTurn`)
  (`self.ChangeSideToTurn`))

(event `InputAction|Interact` :consume false
  (params (Key :type "Key Structure"))
  ;[1 1 1] InputInteract
  (:`Pressed`
    (if (`self.IsActive`)
      (`self.LeaveGame`)
      (elif (and (`self.NeedPlayerAction`) (`self.CanPlayerInteract`))
        (`self.MG_Start`)))))

(event `ActivateDeactivateMouseAndValve`
  (params (Activate :type Boolean))
  (bind _mouse (`self.Mouse`))
  ;[1 1 1] ActivateDeactivateMouse
  (if Activate
    (set `self.MouseActivated` true)
    (`SceneComponent.SetVisibility` _mouse true false)
    (`PrimitiveComponent.SetCollisionProfileName` _mouse "Trigger" true)
    (`PrimitiveComponent.SetCollisionProfileName` (`self.Valve`) "Trigger" true)
    (else
      (set `self.MouseActivated` false)
      (`SceneComponent.SetVisibility` _mouse false false)
      (`PrimitiveComponent.SetCollisionProfileName` _mouse "NoCollision" false)
      (`PrimitiveComponent.SetCollisionProfileName` (`self.Valve`) "NoCollision" false))))

(event `WinGame`
  ;[1 1 1] WinGame
  (set `self.NeedPlayerAction` false)
  (set `self.IsFinished` true)
  (set `self.IsPlaying` false)
  (`/Game/Blueprints/MiniGames/MG_Manager.IncrDecrCurrentGames` (`self.MGManager`) false true)
  (set `self.TimeToWin` (`self.TimeToWinValue`))
  (set `self.StepPassed` 0)
  (`self.LeaveGame`))

(event `InputAction|Attack` :consume false
  (params (Key :type "Key Structure"))
  (bind _mouse (`self.Mouse`))
  ;[1 1 1] InputLeftClick
  (:`Pressed`
    (set `self.LeftClickPressed` true)
    (if (`self.MouseActivated`)
      (`PaperSpriteComponent.SetSprite` _mouse "/Game/Sprites/MiniGames/Chimney_Hand02.Chimney_Hand02")))
  (:`Released`
    (set `self.LeftClickPressed` false)
    (if (`self.MouseActivated`)
      (`PaperSpriteComponent.SetSprite` _mouse "/Game/Sprites/MiniGames/Chimney_Hand01.Chimney_Hand01"))))

(event `LeaveGame`
  (bind _warningbubble (`self.WarningBubble`))
  ;[1 1 1] LeaveGame
  (`self.EnableInput` (`self.Player`) null)
  (set `PlayerController.bShowMouseCursor` false (`GameplayStatics.GetPlayerController` 0))
  (`/Game/Blueprints/Cam.FocusMG` (`self.Cam`) false (0.0 0.0 0.0))
  (`/Game/UI/HUD_Main.ShowWidgets` (`self.HUD`) true)
  (`SceneComponent.K2_SetWorldRotation` (`self.Valve`) (`KismetMathLibrary.MakeRotator` 0.0 (`KismetMathLibrary.RandomFloatInRange` -90.0 90.0)) false false)
  (set `self.LastSprite` (`PaperSpriteComponent.GetSprite` (`self.Chimney_Gauge`)))
  (`self.DisplaySpritesMG` true)
  (`self.ActivateDeactivateMouseAndValve` false)
  (set `self.IsActive` false)
  (`/Engine/EditorBlueprintResources/StandardMacros.IsValid` _warningbubble
    (:`Is Valid`
      (`/Game/Blueprints/MiniGames/WarningBubble.Disappear` _warningbubble)
      (set `self.CanPlayerInteract` false)
      (`self.ChangeSprites` false))))

(event `ChangeSideToTurn`
  (bind _returnvalue (`KismetMathLibrary.RandomInteger` 2))
  (bind _chimney_arrowright (`self.Chimney_ArrowRight`))
  (bind _chimney_arrowleft (`self.Chimney_ArrowLeft`))
  ;[1 1 1] ChangeSiteToTurn
  (if (== _returnvalue 0)
    (set `self.HaveToTurnRight` true)
    (set `self.HaveToTurnLeft` false)
    (`SceneComponent.SetVisibility` _chimney_arrowleft false false)
    (`SceneComponent.SetVisibility` _chimney_arrowright true false)
    (elif (== _returnvalue 1)
      (set `self.HaveToTurnRight` false)
      (set `self.HaveToTurnLeft` true)
      (`SceneComponent.SetVisibility` _chimney_arrowleft true false)
      (`SceneComponent.SetVisibility` _chimney_arrowright false false))))

(event `DisplaySpritesMG`
  (params (Hide :type Boolean))
  (bind _valve (`self.Valve`))
  (bind _chimney_gauge (`self.Chimney_Gauge`))
  ;[1 1 1] DisplaySpriter
  (if Hide
    (`SceneComponent.SetVisibility` _valve false false)
    (`SceneComponent.SetVisibility` _chimney_gauge false false)
    (`SceneComponent.SetVisibility` (`self.Chimney_ArrowRight`) false false)
    (`SceneComponent.SetVisibility` (`self.Chimney_ArrowLeft`) false false)
    (else
      (`SceneComponent.SetVisibility` _valve true false)
      (`SceneComponent.SetVisibility` _chimney_gauge true false)
      (`PaperSpriteComponent.SetSprite` _chimney_gauge (`self.LastSprite`)))))

(event `DifficultySteps`
  (params (DifficultyLevel :type Integer))
  (if (== DifficultyLevel 1)
    (set `self.RotationValueToReach` 30.0)
    (set `self.ValveSpeed` 4.0)
    (set `self.TimeToWinValue` 2.0)
    (set `self.CooldownLoseStep` 1.0)
    (elif (== DifficultyLevel 2)
      (set `self.RotationValueToReach` 40.0)
      (set `self.ValveSpeed` 4.0)
      (set `self.TimeToWinValue` 2.5)
      (set `self.CooldownLoseStep` 0.8)
      (elif (== DifficultyLevel 3)
        (set `self.RotationValueToReach` 50.0)
        (set `self.ValveSpeed` 4.0)
        (set `self.TimeToWinValue` 3.0)
        (set `self.CooldownLoseStep` 0.6)))))

(fn `UserConstructionScript`)