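; Engine repair station minigame on the ship, played as a button-sequence QTE when it needs action and the player is in range.
; Interact opens or leaves it, toggling camera focus, blur widget and player input.
; Correct presses spawn the next random, non-repeating prompt as a runtime flipbook component, while mistakes step back one.
; Tick updates the engine flipbook and detects completion, which decrements MG_Manager's game count and dismisses the warning bubble.
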(event `self.ReceiveActorBeginOverlap`
  (params (OtherActor :type "Actor Object Reference"))
  ;[1 1 1] Collision
  (cast `/Game/Blueprints/Char` OtherActor)
  (if (`self.NeedPlayerAction`)
    (set `self.CanPlayerInteract` true)
    (`PaperFlipbookComponent.SetFlipbook` (`self.EngineFlipbook`) "/Game/Anim/MiniGames/MG_Engine_Interact.MG_Engine_Interact")))

(event `self.ReceiveActorEndOverlap`
  (params (OtherActor :type "Actor Object Reference"))
  ;[1 1 1] Collision
  (cast `/Game/Blueprints/Char` OtherActor)
  (set `self.CanPlayerInteract` false))

(event `self.ReceiveBeginPlay`
  (bind _buttonssprites (`self.ButtonsSprites`))
  ;[0 1 0.2568] Begin Play
  (`|ExecutionSequence`
    (:`then_0`
      (bind _returnvalue (`|CreateWidget` "/Game/UI/MG_Blur.MG_Blur_C"))
      (bind _output_get (set `self.EngineWidget` _returnvalue))
      (`UserWidget.AddToViewport` _output_get 0)
      (`Widget.SetVisibility` _output_get "Hidden")
      (bind _outactors (`GameplayStatics.GetAllActorsOfClass` "/Game/Blueprints/MiniGames/MG_Manager.MG_Manager_C"))
      (set `self.MGManager` (`|GetArrayItem` _outactors))
      (set `self.MGFocusLocOffset` (`self.K2_GetActorLocation`))
      (bind _outactors_2 (`GameplayStatics.GetAllActorsOfClass` "/Game/Blueprints/Ship.Ship_C"))
      (set `self.Ship` (`|GetArrayItem` _outactors_2))
      (bind _outactors_3 (`GameplayStatics.GetAllActorsOfClass` "/Game/Blueprints/Char.Char_C"))
      (set `self.Player` (`|GetArrayItem` _outactors_3)))
    (:`then_1`
      (`KismetArrayLibrary.Array_Add` _buttonssprites (`self.Button0`))
      (`KismetArrayLibrary.Array_Add` _buttonssprites (`self.Button1`))
      (`KismetArrayLibrary.Array_Add` _buttonssprites (`self.Button2`))
      (`KismetArrayLibrary.Array_Add` _buttonssprites (`self.Button3`))
      (`KismetArrayLibrary.Array_Add` _buttonssprites (`self.Button4`))
      (`KismetArrayLibrary.Array_Add` _buttonssprites (`self.Button5`))
      (`self.DisplaySpritesMG` true))))

(event `self.ReceiveTick`
  (params (DeltaSeconds :type "Float (single-precision)"))
  ;[1 0.09001 0.04025] Tick
  (`self.EngineGame`))

(event `LeaveGame`
  (`Widget.SetVisibility` (`self.EngineWidget`) "Hidden")
  (`/Game/Blueprints/Cam.FocusMG` (`/Game/Blueprints/MiniGames/MG_Manager.MainCam` (`self.MGManager`)) false (0.0 0.0 0.0))
  (`self.EnableInput` (`self.Player`) null)
  (`self.ClearQTE`)
  (`self.DisplaySpritesMG` true)
  (set `self.IsActive` false))

(event `StartGame`
  (`Widget.SetVisibility` (`self.EngineWidget`) "Visible")
  (`/Game/Blueprints/Cam.FocusMG` (`/Game/Blueprints/MiniGames/MG_Manager.MainCam` (`self.MGManager`)) true (`self.MGFocusLocOffset`))
  (`/Game/UI/HUD_Main.ShowWidgets` (`/Game/Blueprints/MiniGames/MG_Manager.HUD` (`self.MGManager`)) false)
  (`self.CreateQTE`)
  (`self.DisableInput` (`self.Player`) null)
  (`self.DisplaySpritesMG` false)
  (set `self.IsActive` true))

(event `EngineGame`
  ;[1 0 0.9825] Begin/End game
  (if (`self.NeedPlayerAction`)
    (`|ExecutionSequence`
      (:`then_0`
        (set `self.IsPlaying` true)
        (if (not (`self.CanPlayerInteract`))
          (`PaperFlipbookComponent.SetFlipbook` (`self.EngineFlipbook`) "/Game/Anim/MiniGames/MG_Engine_Warning.MG_Engine_Warning")))
      (:`then_1`
        (if (== (`self.QteDone`) (`self.NumberOfInputs`))
          (`self.EndGame`))))
    (else
      (`PaperFlipbookComponent.SetFlipbook` (`self.EngineFlipbook`) "/Game/Anim/MiniGames/MG_Engine_Idle.MG_Engine_Idle"))))

(event `InputQTE`
  (params (InputValue :type Integer))
  (bind _qtedone (`self.QteDone`))
  (bind _qtedone_2 (`self.QteDone`))
  (bind _output (`|GetArrayItem` (`self.QTEFlipbooks`) _qtedone))
  (bind _output_2 (`|GetArrayItem` (`self.ButtonsSprites`) (`self.QteDone`)))
  (bind _volumemultiplier (`/Game/Blueprints/Ship.VolumeMultiplier` (`self.Ship`)))
  ;[1 1 1] Event INPUT QTE
  (if (`self.IsActive`)
    (if (== (`|GetArrayItem` (`self.QTERandom`) (`self.QteDone`)) InputValue)
      (`PaperFlipbookComponent.SetLooping` _output false)
      (`PaperSpriteComponent.SetSprite` _output_2 "/Game/Sprites/MiniGames/QTE_ButtonOn.QTE_ButtonOn")
      (`/Engine/EditorBlueprintResources/StandardMacros.IncrementInt` _qtedone
        (:`  `
          (`self.CreateQTE`)
          (`PlayerController.ClientPlayCameraShakeFromSource` (`GameplayStatics.GetPlayerController` 0) "/Game/Blueprints/CamShakeMG.CamShakeMG_C" null)
          (`GameplayStatics.PlaySound2D` "/Game/Sound/ButtonEngine_Cue.ButtonEngine_Cue" _volumemultiplier 1.0 0.0 null null)))
      (elif (> _qtedone 0)
        (`ActorComponent.K2_DestroyComponent` _output)
        (`PaperSpriteComponent.SetSprite` _output_2 "/Game/Sprites/MiniGames/QTE_ButtonWrong.QTE_ButtonWrong")
        (`KismetArrayLibrary.Array_Remove` (`self.QTEFlipbooks`) _qtedone_2)
        (`KismetArrayLibrary.Array_Remove` (`self.QTERandom`) _qtedone_2)
        (`/Engine/EditorBlueprintResources/StandardMacros.DecrementInt` _qtedone_2
          (:`  `
            (`/Engine/EditorBlueprintResources/StandardMacros.DecrementInt` (`self.NumberOfQte`)
              (:`  `
                (`PaperFlipbookComponent.Play` _output)
                (`GameplayStatics.PlaySound2D` "/Game/Sound/ButtonEngine_Cue.ButtonEngine_Cue" _volumemultiplier 0.5 0.0 null null)))))))))

(event `InputAction|Attack` :consume false
  (params (Key :type "Key Structure"))
  ;[1 1 1] Inputs
  (:`Pressed`
    (`self.InputQTE` 0)))

(event `InputAction|Interact` :consume false
  (params (Key :type "Key Structure"))
  (:`Pressed`
    (if (`self.IsActive`)
      (`self.LeaveGame`)
      (elif (and (`self.NeedPlayerAction`) (`self.CanPlayerInteract`))
        (`self.StartGame`)))))

(event `Key|Q` :consume false
  (params (Key :type "Key Structure"))
  ;[1 1 1] Inputs
  (:`Pressed`
    (`self.InputQTE` 1)))

(event `Key|Z` :consume false
  (params (Key :type "Key Structure"))
  ;[1 1 1] Inputs
  (:`Pressed`
    (`self.InputQTE` 2)))

(event `EndGame`
  (bind _warningbubble (`self.WarningBubble`))
  ;[1 1 1] Event END GAME
  (set `self.NeedPlayerAction` false)
  (set `self.IsFinished` true)
  (set `self.IsPlaying` false)
  (`/Game/Blueprints/MiniGames/MG_Manager.IncrDecrCurrentGames` (`self.MGManager`) false true)
  (`KismetSystemLibrary.Delay` 0.2)
  (`/Engine/EditorBlueprintResources/StandardMacros.IsValid` _warningbubble
    (:`Is Valid`
      (`/Game/Blueprints/MiniGames/WarningBubble.Disappear` _warningbubble)
      (`self.LeaveGame`)
      (set `self.QteDone` 0))))

(event `DisplaySpritesMG`
  (params (Hide :type Boolean))
  (bind _engine_bg (`self.Engine_BG`))
  (if Hide
    (`PaperSpriteComponent.SetSprite` _engine_bg null)
    (for _array_element (`self.ButtonsSprites`)
      (`PaperSpriteComponent.SetSprite` _array_element null))
    (else
      (`PaperSpriteComponent.SetSprite` _engine_bg "/Game/Sprites/MiniGames/QTE_BG.QTE_BG")
      (for _array_element_2 (`self.ButtonsSprites`)
        (`PaperSpriteComponent.SetSprite` _array_element_2 "/Game/Sprites/MiniGames/QTE_ButtonOff.QTE_ButtonOff")))))

(event `CreateQTE`
  (bind _returnvalue (`KismetMathLibrary.RandomInteger` 3))
  (bind _zvalueqteinputs (`self.ZValueQteInputs`))
  (bind _numberofqte (`self.NumberOfQte`))
  (bind _qtedone (`self.QteDone`))
  (bind _returnvalue_2 (- (`self.NumberOfQte`) 1))
  (bind _output (`|GetArrayItem` (`self.QTEFlipbooks`) _returnvalue_2))
  (bind _output_2 (`|GetArrayItem` (`self.QTERandom`) _returnvalue_2))
  (bind _returnvalue_3 (- (* _returnvalue_2 (`self.xMultiplicator`)) 65.0))
  ;[1 1 1] CREATE QTE
  (if (not (== _numberofqte (`self.NumberOfInputs`)))
    (`/Engine/EditorBlueprintResources/StandardMacros.IncrementInt` _numberofqte
      (:`  `
        (bind _returnvalue_4 (`AddComponent|NODE_AddPaperFlipbookComponent-1`))
        (`KismetArrayLibrary.Array_Add` (`self.QTEFlipbooks`) _returnvalue_4)
        (`KismetArrayLibrary.Array_Add` (`self.QTERandom`) _returnvalue)
        (set `self.NewQteNumber` _returnvalue)
        (if (> _qtedone 0)
          (while (== (`self.NewQteNumber`) (`|GetArrayItem` (`self.QTERandom`) (- _qtedone 1)))
            (set `self.NewQteNumber` (`KismetMathLibrary.RandomInteger` 3)))
          (`KismetArrayLibrary.Array_Set` (`self.QTERandom`) (- (`self.NumberOfQte`) 1) (`self.NewQteNumber`)))
        (if (== _output_2 0)
          (`SceneComponent.K2_SetRelativeLocation` _output (`KismetMathLibrary.MakeVector` _returnvalue_3 24.0 _zvalueqteinputs) false false)
          (`SceneComponent.SetWorldScale3D` _output (2.0 1.0 2.0))
          (`PaperFlipbookComponent.SetFlipbook` _output "/Game/Anim/MiniGames/QTE_FlipLeftClick.QTE_FlipLeftClick")
          (elif (== _output_2 1)
            (`SceneComponent.K2_SetRelativeLocation` _output (`KismetMathLibrary.MakeVector` _returnvalue_3 25.0 _zvalueqteinputs) false false)
            (`SceneComponent.SetWorldScale3D` _output (2.0 1.0 2.0))
            (`PaperFlipbookComponent.SetFlipbook` _output "/Game/Anim/MiniGames/QTE_FlipQ.QTE_FlipQ")
            (elif (== _output_2 2)
              (`SceneComponent.K2_SetRelativeLocation` _output (`KismetMathLibrary.MakeVector` _returnvalue_3 25.0 _zvalueqteinputs) false false)
              (`SceneComponent.SetWorldScale3D` _output (2.0 1.0 2.0))
              (`PaperFlipbookComponent.SetFlipbook` _output "/Game/Anim/MiniGames/QTE_FlipZ.QTE_FlipZ"))))))))

(event `ClearQTE`
  (bind _qteflipbooks (`self.QTEFlipbooks`))
  ;[1 1 1] CREATE QTE
  ;;[1 1 1] CLEAR QTE
  (`KismetArrayLibrary.Array_Clear` (`self.QTERandom`))
  (set `self.NumberOfQte` 0)
  (set `self.QteDone` 0)
  (for _array_element _qteflipbooks
    (`ActorComponent.K2_DestroyComponent` _array_element))
  (`KismetArrayLibrary.Array_Clear` _qteflipbooks))

(fn `UserConstructionScript`)