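; TNT button-mashing minigame actor on the Ship, flagged by NeedPlayerAction and opened or left with Interact while the character overlaps it.
; Entering shows the spam bar, focuses the manager's camera, hides the HUD and disables jumping.
; Jump presses fill progress, with sound and camera shake, against a constant drain in Tick; DifficultySteps tunes both rates.
; A full bar finishes the game, updates MG_Manager and clears the warning bubble.
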(event `self.ReceiveBeginPlay`
  ;[1 1 1] BeginPlay
  (bind _returnvalue (`|CreateWidget` "/Game/UI/MG_SpamBar.MG_SpamBar_C"))
  (bind _output_get (set `self.SpamBar` _returnvalue))
  (`UserWidget.AddToViewport` _output_get 0)
  (`Widget.SetVisibility` _output_get "Hidden")
  (bind _outactors (`GameplayStatics.GetAllActorsOfClass` "/Game/Blueprints/MiniGames/MG_Manager.MG_Manager_C"))
  (set `self.MG_Manager` (`|GetArrayItem` _outactors))
  (set `self.MGFocusLocOffset` (`self.K2_GetActorLocation`))
  (`self.SetImage` 8)
  (bind _outactors_2 (`GameplayStatics.GetAllActorsOfClass` "/Game/Blueprints/Ship.Ship_C"))
  (set `self.Ship` (`|GetArrayItem` _outactors_2)))

(event `self.ReceiveTick`
  (params (DeltaSeconds :type "Float (single-precision)"))
  ;[1 1 1] Tick
  (`|ExecutionSequence`
    (:`then_0`
      (`self.SpamGameEvent` DeltaSeconds))
    (:`then_1`
      (set `self.SpamCurrentValuePerc` (- (`self.SpamCurrentValuePerc`) (/ DeltaSeconds (`self.Dividor`)))))))

(event `SpamGameEvent`
  (params (DeltaTime :type "Float (double-precision)"))
  (bind _paperflipbook (`self.PaperFlipbook`))
  (bind _warningbubble (`self.WarningBubble`))
  (bind _returnvalue (`KismetMathLibrary.NearlyEqual_FloatFloat` (`self.SpamCurrentValuePerc`) 1.0 0.01))
  ;[1 1 1] EventSpamGame
  (if (`self.NeedPlayerAction`)
    (`|ExecutionSequence`
      (:`then_0`
        (set `self.IsPlaying` true)
        (if (not (`self.CanPlayerInteract`))
          (`PaperFlipbookComponent.SetFlipbook` _paperflipbook "/Game/Anim/MiniGames/MiniGameTNT.MiniGameTNT")))
      (:`then_1`
        (if (`self.HasWon`)
          _
          (elif _returnvalue
            (set `self.HasWon` _returnvalue)
            (set `self.NeedPlayerAction` false)
            (`Widget.SetVisibility` (`self.SpamBar`) "Hidden")
            (`/Game/Blueprints/Cam.FocusMG` (`/Game/Blueprints/MiniGames/MG_Manager.MainCam` (`self.MG_Manager`)) false (0.0 0.0 0.0))
            (`/Game/UI/HUD_Main.ShowWidgets` (`/Game/Blueprints/MiniGames/MG_Manager.HUD` (`self.MG_Manager`)) true)
            (set `self.HasWon` false)
            (set `self.IsFinished` true)
            (set `self.IsPlaying` false)
            (`/Game/Blueprints/MiniGames/MG_Manager.IncrDecrCurrentGames` (`self.MG_Manager`) false true)
            (`self.LeaveGame`)
            (`/Engine/EditorBlueprintResources/StandardMacros.IsValid` _warningbubble
              (:`Is Valid`
                (`/Game/Blueprints/MiniGames/WarningBubble.Disappear` _warningbubble)))))))
    (else
      (`PaperFlipbookComponent.SetFlipbook` _paperflipbook "/Game/Anim/MiniGames/MG_Explosive_Idle.MG_Explosive_Idle"))))

(event `InputAction|Jump` :consume false
  (params (Key :type "Key Structure"))
  ;[1 1 1] Input Space
  (:`Pressed`
    (if (`self.NeedPlayerAction`)
      (if (`self.CanPlayerInteract`)
        (set `self.SpamCurrentValuePerc` (`KismetMathLibrary.FClamp` (+ (/ (`self.SpamValue`) (`self.SpamTotalValue`)) (`self.SpamCurrentValuePerc`))))
        (set `/Game/UI/MG_SpamBar.PressSpace` true (`self.SpamBar`))
        (`GameplayStatics.PlaySound2D` "/Game/Sound/MG_TNT_Boot.MG_TNT_Boot" (`/Game/Blueprints/Ship.VolumeMultiplier` (`self.Ship`)) 1.0 0.0 null null)
        (`PlayerController.ClientPlayCameraShakeFromSource` (`GameplayStatics.GetPlayerController` 0) "/Game/Blueprints/CamShakeMG.CamShakeMG_C" null))))
  (:`Released`
    (set `/Game/UI/MG_SpamBar.PressSpace` false (`self.SpamBar`))
    (`PlayerController.ClientStopCameraShake` (`GameplayStatics.GetPlayerController` 0) "/Game/Blueprints/CamShakeMG.CamShakeMG_C" true)))

(event `self.ReceiveActorBeginOverlap`
  (params (OtherActor :type "Actor Object Reference"))
  ;[1 1 1] Collision
  (if (`self.NeedPlayerAction`)
    (cast `/Game/Blueprints/Char` OtherActor)
    (set `self.CanPlayerInteract` true)
    (`PaperFlipbookComponent.SetFlipbook` (`self.PaperFlipbook`) "/Game/Anim/MiniGames/MG_TNT_Interact.MG_TNT_Interact")))

(event `self.ReceiveActorEndOverlap`
  (params (OtherActor :type "Actor Object Reference"))
  ;[1 1 1] Collision
  (cast `/Game/Blueprints/Char` OtherActor)
  (set `self.CanPlayerInteract` false))

(event `StartGame`
  ;[1 1 1] EnterGame
  (`Widget.SetVisibility` (`self.SpamBar`) "Visible")
  (`/Game/Blueprints/Cam.FocusMG` (`/Game/Blueprints/MiniGames/MG_Manager.MainCam` (`self.MG_Manager`)) true (`self.MGFocusLocOffset`))
  (`/Game/UI/HUD_Main.ShowWidgets` (`/Game/Blueprints/MiniGames/MG_Manager.HUD` (`self.MG_Manager`)) false)
  (set `self.IsActive` true)
  (set `Character.JumpMaxCount` 0 (`GameplayStatics.GetPlayerCharacter` 0)))

(event `LeaveGame`
  ;[1 1 1] LeaveGame
  (`Widget.SetVisibility` (`self.SpamBar`) "Hidden")
  (`/Game/Blueprints/Cam.FocusMG` (`/Game/Blueprints/MiniGames/MG_Manager.MainCam` (`self.MG_Manager`)) false (0.0 0.0 0.0))
  (set `self.IsActive` false)
  (`KismetSystemLibrary.Delay` 0.3)
  (set `Character.JumpMaxCount` 1 (`GameplayStatics.GetPlayerCharacter` 0)))

(event `InputAction|Interact` :consume false
  (params (Key :type "Key Structure"))
  ;[1 1 1] RightClick
  (:`Pressed`
    (if (`self.IsActive`)
      (`self.LeaveGame`)
      (elif (and (`self.NeedPlayerAction`) (`self.CanPlayerInteract`))
        (`self.StartGame`)))))

(event `DifficultySteps`
  (params (DifficultyLevel :type Integer))
  (if (== DifficultyLevel 1)
    (set `self.Dividor` 1.5)
    (set `self.SpamValue` 15.0)
    (elif (== DifficultyLevel 2)
      (set `self.Dividor` 1.2)
      (set `self.SpamValue` 10.0)
      (elif (== DifficultyLevel 3)
        (set `self.Dividor` 1.0)
        (set `self.SpamValue` 9.0)))))

(fn `SetImage`
  (params (DelayValue :type Integer))
  (bind _foundwidgets (`WidgetBlueprintLibrary.GetAllWidgetsOfClass` "/Game/UI/MG_SpamBar.MG_SpamBar_C"))
  (for _array_element _foundwidgets
    (set `/Game/UI/MG_SpamBar.Delay` DelayValue _array_element)
    (`Image.SetColorAndOpacity` (`/Game/UI/MG_SpamBar.AnimSpam` _array_element) (struct :`R` 1.0 :`G` 1.0 :`B` 1.0 :`A` 1.0))))

(fn `UserConstructionScript`)