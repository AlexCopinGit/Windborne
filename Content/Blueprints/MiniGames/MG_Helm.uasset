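; Helm steering minigame actor that the player joins with Interact when it needs action, switching camera focus, HUD and player input.
; While active, a random drift rotates the helm sprite against MoveRight input, and each tick BoxHelm overlaps BoxBG adds score.
; Reaching the difficulty-scaled MaxScore, or pressing Interact again, ends it as a win and decrements the manager's game count.
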(event `self.ReceiveActorBeginOverlap`
  (params (OtherActor :type "Actor Object Reference"))
  (cast `/Game/Blueprints/Char` OtherActor)
  (if (`self.NeedPlayerAction`)
    (set `self.CanPlayerInteract` true)
    (`PaperFlipbookComponent.SetFlipbook` (`self.PaperFlipbook`) "/Game/Anim/MiniGames/MG_Helm_Interact.MG_Helm_Interact")))

(event `self.ReceiveActorEndOverlap`
  (params (OtherActor :type "Actor Object Reference"))
  (cast `/Game/Blueprints/Char` OtherActor)
  (set `self.CanPlayerInteract` false))

(event `InputAction|Interact` :consume false
  (params (Key :type "Key Structure"))
  (:`Pressed`
    (if (`self.IsActive`)
      (`self.End`)
      (elif (and (`self.NeedPlayerAction`) (`self.CanPlayerInteract`))
        (`self.Join`)))))

(event `self.ReceiveBeginPlay`
  (bind _returnvalue (`|CreateWidget` "/Game/UI/MG_Blur.MG_Blur_C"))
  (bind _output_get (set `self.Widget` _returnvalue))
  (`UserWidget.AddToViewport` _output_get 0)
  (`Widget.SetVisibility` _output_get "Hidden")
  (bind _outactors (`GameplayStatics.GetAllActorsOfClass` "/Game/Blueprints/Ship.Ship_C"))
  (set `self.Ship` (`|GetArrayItem` _outactors))
  (bind _outactors_2 (`GameplayStatics.GetAllActorsOfClass` "/Game/Blueprints/Char.Char_C"))
  (set `self.Player` (`|GetArrayItem` _outactors_2))
  (bind _outactors_3 (`GameplayStatics.GetAllActorsOfClass` "/Game/Blueprints/MiniGames/MG_Manager.MG_Manager_C"))
  (set `self.MGManager` (`|GetArrayItem` _outactors_3))
  (set `self.LocOffset` (`self.K2_GetActorLocation`)))

(event `self.ReceiveTick`
  (params (DeltaSeconds :type "Float (single-precision)"))
  (bind _paperflipbook (`self.PaperFlipbook`))
  (`|ExecutionSequence`
    (:`then_0`
      (if (`self.NeedPlayerAction`)
        (set `self.IsPlaying` true)
        (if (not (`self.CanPlayerInteract`))
          (`PaperFlipbookComponent.SetFlipbook` _paperflipbook "/Game/Anim/MiniGames/MG_Helm_Warning.MG_Helm_Warning"))
        (else
          (`PaperFlipbookComponent.SetFlipbook` _paperflipbook "/Game/Anim/MiniGames/MG_Helm_Idle.MG_Helm_Idle"))))
    (:`then_1`
      (if (`self.IsActive`)
        (`|ExecutionSequence`
          (:`then_0`
            (`self.GameplayLoop`))
          (:`then_1`
            (if (`self.IsTurningHelm`)
              (`KismetSystemLibrary.Delay` 1.0)
              (`GameplayStatics.PlaySound2D` "/Game/Sound/Minigame_wood.Minigame_wood" (`/Game/Blueprints/Ship.VolumeMultiplier` (`self.Ship`)) 1.0 0.0 null null))))))))

(event `Join`
  (`Widget.SetVisibility` (`self.Widget`) "Visible")
  (`/Game/Blueprints/Cam.FocusMG` (`/Game/Blueprints/MiniGames/MG_Manager.MainCam` (`self.MGManager`)) true (`self.LocOffset`))
  (`/Game/UI/HUD_Main.ShowWidgets` (`/Game/Blueprints/MiniGames/MG_Manager.HUD` (`self.MGManager`)) false)
  (`self.DisableInput` (`self.Player`) null)
  (set `self.IsActive` true)
  (`self.Start`))

(event `Leave`
  (bind _warningbubble (`self.WarningBubble`))
  (`Widget.SetVisibility` (`self.Widget`) "Hidden")
  (`/Game/Blueprints/Cam.FocusMG` (`/Game/Blueprints/MiniGames/MG_Manager.MainCam` (`self.MGManager`)) false (0.0 0.0 0.0))
  (`self.EnableInput` (`self.Player`) null)
  (set `self.IsActive` false)
  (`/Engine/EditorBlueprintResources/StandardMacros.IsValid` _warningbubble
    (:`Is Valid`
      (`/Game/Blueprints/MiniGames/WarningBubble.Disappear` _warningbubble))))

(event `Win`
  (set `self.NeedPlayerAction` false)
  (set `self.IsFinished` true)
  (set `self.IsPlaying` false)
  (`/Game/Blueprints/MiniGames/MG_Manager.IncrDecrCurrentGames` (`self.MGManager`) false true)
  (`self.Leave`))

(event `Start`
  (`SceneComponent.SetVisibility` (`self.Sprite_BG`) true false)
  (`SceneComponent.SetVisibility` (`self.Sprite_Helm`) true false)
  (bind _output_get (set `self.RotOffRand` (`KismetMathLibrary.RandomIntegerInRange` -1 1) :!label _label))
  (if (== _output_get 0)
    (goto _label)
    (else
      (`SceneComponent.K2_SetWorldRotation` (`self.Sprite_Helm`) (`KismetMathLibrary.MakeRotator` 0.0 (* _output_get (`self.RotOffValue`))) false false)
      (set `self.Score` 0.0))))

(event `End`
  (`SceneComponent.SetVisibility` (`self.Sprite_BG`) false false)
  (`SceneComponent.SetVisibility` (`self.Sprite_Helm`) false false)
  (`self.Win`))

(event `GameplayLoop`
  (bind _returnvalue (/ (`self.TurnAxis`) 3.0))
  (`|ExecutionSequence`
    (:`then_0`
      (`SceneComponent.K2_AddWorldRotation` (`self.Sprite_Helm`) (`KismetMathLibrary.MakeRotator` 0.0 (- (/ (`self.RandAxis`) 3.0) (* _returnvalue (`self.TurnForce`)))) false false)
      (if (!= _returnvalue 0.0)
        (set `self.IsTurningHelm` false)
        (else
          (set `self.IsTurningHelm` true))))
    (:`then_1`
      (`KismetSystemLibrary.Delay` (`self.RandInterval`))
      (`GameplayStatics.PlaySound2D` "/Game/Sound/Minigame_wood__1_.Minigame_wood__1_" (`/Game/Blueprints/Ship.VolumeMultiplier` (`self.Ship`)) 0.5 0.0 null null)
      (bind _output_get (set `self.RandAxis` (`KismetMathLibrary.Conv_IntToDouble` (`KismetMathLibrary.RandomIntegerInRange` -1 1)) :!label _label_2))
      (if (== _output_get 0.0)
        (goto _label_2)))
    (:`then_2`
      (if (`PrimitiveComponent.IsOverlappingComponent` (`self.Box_Helm`) (`self.Box_BG`))
        (set `self.Score` (+ (`self.Score`) 1.0))
        (if (>= (`self.Score`) (`self.MaxScore`))
          (`self.End`))))))

(event `InputAxis|MoveRight` :consume false
  (params (AxisValue :type "Float (single-precision)"))
  (set `self.TurnAxis` AxisValue))

(event `DifficultySteps`
  (params (DifficultyLevel :type Integer))
  (if (== DifficultyLevel 1)
    (set `self.RandInterval` 0.8)
    (set `self.MaxScore` 300.0)
    (set `self.TurnForce` 1.7)
    (elif (== DifficultyLevel 2)
      (set `self.RandInterval` 0.7)
      (set `self.MaxScore` 400.0)
      (set `self.TurnForce` 1.5)
      (elif (== DifficultyLevel 3)
        (set `self.RandInterval` 0.7)
        (set `self.MaxScore` 500.0)
        (set `self.TurnForce` 1.4)))))

(fn `UserConstructionScript`)