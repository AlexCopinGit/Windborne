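; Alembic minigame actor the player starts when it needs action, focusing the camera, disabling player input and hiding the HUD.
; Tick slides the glass back and forth; Attack spawns one drop sprite at its position, and per-tick overlap polling scores or discards it.
; Each hit randomly moves the blue bar; enough hits award Ship time and update MG_Manager's game count.
; DifficultySteps scales required drops and glass speed, while leaving resets progress.
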(event `self.ReceiveActorBeginOverlap`
  (params (OtherActor :type "Actor Object Reference"))
  ;[1 1 1] Collision
  (if (`self.NeedPlayerAction`)
    (cast `/Game/Blueprints/Char` OtherActor)
    (set `self.CanPlayerInteract` true)
    (`PaperFlipbookComponent.SetFlipbook` (`self.AlambicFlipbook`) "/Game/Anim/MiniGames/AlambicInteract.AlambicInteract")))

(event `self.ReceiveActorEndOverlap`
  (params (OtherActor :type "Actor Object Reference"))
  ;[1 1 1] Collision
  (cast `/Game/Blueprints/Char` OtherActor)
  (set `self.CanPlayerInteract` false))

(event `self.ReceiveBeginPlay`
  ;[1 1 1] BeginPlay
  (`|ExecutionSequence`
    (:`then_0`
      (`self.DisplaySprites` true)
      (set `self.GlassPosX` -30.0))
    (:`then_1`
      (bind _outactors (`GameplayStatics.GetAllActorsOfClass` "/Game/Blueprints/MG_Manager.MG_Manager_C"))
      (set `self.MGManager` (`|GetArrayItem` _outactors))
      (set `self.MGFocusLocOffset` (`self.K2_GetActorLocation`))
      (bind _outactors_2 (`GameplayStatics.GetAllActorsOfClass` "/Game/Blueprints/Ship.Ship_C"))
      (set `self.Ship` (`|GetArrayItem` _outactors_2))
      (bind _outactors_3 (`GameplayStatics.GetAllActorsOfClass` "/Game/Blueprints/Char.Char_C"))
      (set `self.Player` (`|GetArrayItem` _outactors_3)))))

(event `InputAction|Attack` :consume false
  (params (Key :type "Key Structure"))
  (:`Pressed`
    (if (`self.IsActive`)
      (if (not (`KismetSystemLibrary.IsValid` (`self.Drop`)))
        (bind _returnvalue (`AddComponent|NODE_AddPaperSpriteComponent-0`))
        (bind _output_get (set `self.Drop` _returnvalue))
        (`SceneComponent.K2_SetWorldLocation` _output_get (`SceneComponent.K2_GetComponentLocation` (`self.Alambic_Glass`)) false false)
        (`PaperSpriteComponent.SetSprite` (`self.Alambic_Glass`) "/Game/Sprites/MiniGames/Alambic_Glass02.Alambic_Glass02")
        (`GameplayStatics.PlaySound2D` (`self.SoundDropAlambic`) (`/Game/Blueprints/Ship.VolumeMultiplier` (`self.Ship`)) 1.0 0.0 null null)))))

(event `self.ReceiveTick`
  (params (DeltaSeconds :type "Float (single-precision)"))
  (bind _glassposx (`self.GlassPosX`))
  (bind _returnvalue (* DeltaSeconds (`self.DeltaTimeMultiplicator`)))
  (`|ExecutionSequence`
    (:`then_0`
      (`self.GameplayLoop`))
    (:`then_1`
      (`SceneComponent.K2_SetRelativeLocation` (`self.Alambic_Glass`) (`KismetMathLibrary.MakeVector` (`self.GlassPosX`) 5.0 21.0) false false))
    (:`then_2`
      (if (<= _glassposx -30.0)
        (set `self.+` true)))
    (:`then_3`
      (if (>= _glassposx 40.0)
        (set `self.+` false)))
    (:`then_4`
      (if (`self.+`)
        (set `self.GlassPosX` (+ (`self.GlassPosX`) _returnvalue))
        (else
          (set `self.GlassPosX` (- (`self.GlassPosX`) _returnvalue)))))))

(event `DropDrop`
  ;[1 1 1] DropDrop
  (if (`KismetSystemLibrary.IsValid` (`self.Drop`))
    (if (`PrimitiveComponent.IsOverlappingComponent` (`self.Drop`) (`self.TriggerDestroyDrop`))
      (`ActorComponent.K2_DestroyComponent` (`self.Drop`))
      (set `self.Drop` null)
      (`/Engine/EditorBlueprintResources/StandardMacros.IncrementInt` (`self.DropsPut`)
        (:`  `
          (`PaperSpriteComponent.SetSprite` (`self.Alambic_Glass`) "/Game/Sprites/MiniGames/Alambic_Glass01.Alambic_Glass01")
          (`SceneComponent.K2_SetRelativeLocation` (`self.Alambic_Bluebar`) (`KismetMathLibrary.MakeVector` (`KismetMathLibrary.RandomFloatInRange` -22.0 22.0) 1.0 1.0) true false)
          (if (>= (`self.DropsPut`) (`self.DropsNeeded`))
            (`self.WinGame`))))
      (elif (or (`PrimitiveComponent.IsOverlappingComponent` (`self.Drop`) (`self.BadTrigger`)) (`PrimitiveComponent.IsOverlappingComponent` (`self.Drop`) (`self.BadTrigger2`)))
        (`ActorComponent.K2_DestroyComponent` (`self.Drop`))
        (set `self.Drop` null)
        (`PaperSpriteComponent.SetSprite` (`self.Alambic_Glass`) "/Game/Sprites/MiniGames/Alambic_Glass01.Alambic_Glass01")))))

(event `GameplayLoop`
  (if (`self.NeedPlayerAction`)
    (`|ExecutionSequence`
      (:`then_0`
        (set `self.IsPlaying` true)
        (if (not (`self.CanPlayerInteract`))
          (`PaperFlipbookComponent.SetFlipbook` (`self.AlambicFlipbook`) "/Game/Anim/MiniGames/AlambicWarning.AlambicWarning")))
      (:`then_1`
        (`self.DropDrop`)))
    (else
      (`PaperFlipbookComponent.SetFlipbook` (`self.AlambicFlipbook`) "/Game/Anim/MiniGames/AlambicIdle.AlambicIdle"))))

(event `InputAction|Interact` :consume false
  (params (Key :type "Key Structure"))
  ;[1 1 1] RightClick
  (:`Pressed`
    (if (`self.IsActive`)
      (`self.LeaveGame`)
      (elif (and (`self.NeedPlayerAction`) (`self.CanPlayerInteract`))
        (`self.StartGame`)))))

(event `DifficultySteps`
  (params (DifficultyLevel :type Integer))
  (if (== DifficultyLevel 1)
    (set `self.DropsNeeded` 2)
    (set `self.DeltaTimeMultiplicator` 40.0)
    (elif (== DifficultyLevel 2)
      (set `self.DropsNeeded` 3)
      (set `self.DeltaTimeMultiplicator` 50.0)
      (elif (== DifficultyLevel 3)
        (set `self.DropsNeeded` 4)
        (set `self.DeltaTimeMultiplicator` 60.0)))))

(event `StartGame`
  ;[1 1 1] StartGame
  (`/Game/Blueprints/Cam.FocusMG` (`/Game/Blueprints/MG_Manager.MainCam` (`self.MGManager`)) true (`self.MGFocusLocOffset`))
  (`/Game/UI/HUD_Main.ShowWidgets` (`/Game/Blueprints/MG_Manager.HUD` (`self.MGManager`)) false)
  (`self.DisableInput` (`self.Player`) null)
  (`SceneComponent.K2_SetRelativeLocation` (`self.Alambic_Bluebar`) (`KismetMathLibrary.MakeVector` (`KismetMathLibrary.RandomFloatInRange` -22.0 22.0) 1.0 1.0) false false)
  (`self.DisplaySprites` false)
  (set `self.IsActive` true))

(event `LeaveGame`
  (bind _warningbubble (`self.WarningBubble`))
  ;[1 1 1] LeaveGame
  (`/Game/Blueprints/Cam.FocusMG` (`/Game/Blueprints/MG_Manager.MainCam` (`self.MGManager`)) false (0.0 0.0 0.0))
  (`self.EnableInput` (`self.Player`) null)
  (`self.DisplaySprites` true)
  (set `self.IsActive` false)
  (`/Game/UI/HUD_Main.ShowWidgets` (`/Game/Blueprints/MG_Manager.HUD` (`self.MGManager`)) true)
  (set `self.DropsPut` 0)
  (`/Engine/EditorBlueprintResources/StandardMacros.IsValid` _warningbubble
    (:`Is Valid`
      (`/Game/Blueprints/WarningBubble.Disappear` _warningbubble))))

(event `WinGame`
  ;[1 1 1] WinGame
  (set `self.NeedPlayerAction` false)
  (`/Game/Blueprints/Ship.AddTimeGain` (`self.Ship`))
  (set `self.IsFinished` true)
  (set `self.IsPlaying` false)
  (`/Game/Blueprints/MG_Manager.IncrDecrCurrentGames` (`self.MGManager`) false true)
  (`self.LeaveGame`))

(event `DisplaySprites`
  (params (Hide :type Boolean))
  (bind _alambic_bg (`self.Alambic_BG`))
  (bind _alambic_bluebar (`self.Alambic_Bluebar`))
  (bind _alambic_glass (`self.Alambic_Glass`))
  (bind _alambic_bar (`self.Alambic_Bar`))
  ;[1 1 1] DisplaySprites
  (if Hide
    (`PaperSpriteComponent.SetSprite` _alambic_bg null)
    (`PaperSpriteComponent.SetSprite` _alambic_bar null)
    (`PaperSpriteComponent.SetSprite` _alambic_bluebar null)
    (`PaperSpriteComponent.SetSprite` _alambic_glass null)
    (else
      (`PaperSpriteComponent.SetSprite` _alambic_bg "/Game/Sprites/MiniGames/Alambic_Background.Alambic_Background")
      (`PaperSpriteComponent.SetSprite` _alambic_bar "/Game/Sprites/MiniGames/Alambic_Bar.Alambic_Bar")
      (`PaperSpriteComponent.SetSprite` _alambic_bluebar "/Game/Sprites/MiniGames/Alambic_Bluebar.Alambic_Bluebar")
      (`PaperSpriteComponent.SetSprite` _alambic_glass "/Game/Sprites/MiniGames/Alambic_Glass01.Alambic_Glass01"))))

(fn `UserConstructionScript`)