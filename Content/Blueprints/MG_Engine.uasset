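; Engine minigame actor: when it needs player action, an overlapping Char can interact to play a quick-time sequence.
; StartGame shows the widget, focuses the camera, disables player input and spawns random left-click, Q or Z prompt flipbooks one at a time.
; A correct input adds the next prompt; a wrong one steps back one.
; Tick updates warning/idle visuals and ends the completed game, adding Ship time and updating MG_Manager's count.
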(event `self.ReceiveActorBeginOverlap`
  (params (OtherActor :type "Actor Object Reference"))
  ;[1 1 1] Collision
  (cast `/Game/Blueprints/Char` OtherActor)
  (if (`self.NeedPlayerAction`)
    (set `self.CanPlayerInteract` true)
    (`PaperFlipbookComponent.SetFlipbook` (`self.EngineFlipbook`) "/Game/Anim/MiniGames/MG_Engine_Interact.MG_Engine_Interact")))

(event `self.ReceiveActorEndOverlap`
  (params (OtherActor :type "Actor Object Reference"))
  ;[1 1 1] Collision
  (cast `/Game/Blueprints/Char` OtherActor)
  (set `self.CanPlayerInteract` false))

(event `self.ReceiveBeginPlay`
  ;[0 1 0.2568] Begin Play
  (`|ExecutionSequence`
    (:`then_0`
      (bind _returnvalue (`|CreateWidget` "/Game/UI/MG_Engine.MG_Engine_C"))
      (bind _output_get (set `self.EngineWidget` _returnvalue))
      (`UserWidget.AddToViewport` _output_get 0)
      (`Widget.SetVisibility` _output_get "Hidden")
      (bind _outactors (`GameplayStatics.GetAllActorsOfClass` "/Game/Blueprints/MG_Manager.MG_Manager_C"))
      (set `self.MGManager` (`|GetArrayItem` _outactors))
      (set `self.MGFocusLocOffset` (`self.K2_GetActorLocation`))
      (bind _outactors_2 (`GameplayStatics.GetAllActorsOfClass` "/Game/Blueprints/Ship.Ship_C"))
      (set `self.Ship` (`|GetArrayItem` _outactors_2))
      (bind _outactors_3 (`GameplayStatics.GetAllActorsOfClass` "/Game/Blueprints/Char.Char_C"))
      (set `self.Player` (`|GetArrayItem` _outactors_3)))))

(event `self.ReceiveTick`
  (params (DeltaSeconds :type "Float (single-precision)"))
  ;[1 0.09001 0.04025] Tick
  (`self.EngineGame`))

(event `LeaveGame`
  (`Widget.SetVisibility` (`self.EngineWidget`) "Hidden")
  (`/Game/Blueprints/Cam.FocusMG` (`/Game/Blueprints/MG_Manager.MainCam` (`self.MGManager`)) false (0.0 0.0 0.0))
  (`self.EnableInput` (`self.Player`) null)
  (`self.ClearQTE`)
  (set `self.IsActive` false))

(event `StartGame`
  (`Widget.SetVisibility` (`self.EngineWidget`) "Visible")
  (`/Game/Blueprints/Cam.FocusMG` (`/Game/Blueprints/MG_Manager.MainCam` (`self.MGManager`)) true (`self.MGFocusLocOffset`))
  (`/Game/UI/HUD_Main.ShowWidgets` (`/Game/Blueprints/MG_Manager.HUD` (`self.MGManager`)) false)
  (`self.CreateQTE`)
  (`self.DisableInput` (`self.Player`) null)
  (set `self.IsActive` true))

(event `EngineGame`
  ;[1 0 0.9825] Begin/End game
  (if (`self.NeedPlayerAction`)
    (`|ExecutionSequence`
      (:`then_0`
        (set `self.IsPlaying` true)
        (if (not (`self.CanPlayerInteract`))
          (`PaperFlipbookComponent.SetFlipbook` (`self.EngineFlipbook`) "/Game/Anim/MiniGames/MG_Engine_Warning.MG_Engine_Warning")))
      (:`then_1`
        (if (== (`self.QteDone`) (`self.NumberOfInputs`))
          (`self.EndGame`))))
    (else
      (`PaperFlipbookComponent.SetFlipbook` (`self.EngineFlipbook`) "/Game/Anim/MiniGames/MG_Engine_Idle.MG_Engine_Idle"))))

(event `InputQTE`
  (params (InputValue :type Integer))
  (bind _qtedone (`self.QteDone`))
  (bind _qtedone_2 (`self.QteDone`))
  (bind _output (`|GetArrayItem` (`self.QTEFlipbooks`) _qtedone))
  ;[1 1 1] Event INPUT QTE
  (if (`self.IsActive`)
    (if (== (`|GetArrayItem` (`self.QTERandom`) (`self.QteDone`)) InputValue)
      (`PaperFlipbookComponent.Stop` _output)
      (`/Engine/EditorBlueprintResources/StandardMacros.IncrementInt` _qtedone
        (:`  `
          (`self.CreateQTE`)
          (`/Game/Blueprints/Char.EventAttack` (`self.Player`))))
      (elif (> _qtedone 0)
        (`ActorComponent.K2_DestroyComponent` _output)
        (`KismetArrayLibrary.Array_Remove` (`self.QTEFlipbooks`) _qtedone_2)
        (`KismetArrayLibrary.Array_Remove` (`self.QTERandom`) _qtedone_2)
        (`/Engine/EditorBlueprintResources/StandardMacros.DecrementInt` _qtedone_2
          (:`  `
            (`/Engine/EditorBlueprintResources/StandardMacros.DecrementInt` (`self.NumberOfQte`)
              (:`  `
                (`PaperFlipbookComponent.Play` _output)))))))))

(event `InputAction|Attack` :consume false
  (params (Key :type "Key Structure"))
  ;[1 1 1] Inputs
  (:`Pressed`
    (`self.InputQTE` 0)))

(event `InputAction|Interact` :consume false
  (params (Key :type "Key Structure"))
  (:`Pressed`
    (if (`self.IsActive`)
      (`self.LeaveGame`)
      (elif (and (`self.NeedPlayerAction`) (`self.CanPlayerInteract`))
        (`self.StartGame`)))))

(event `Key|Q` :consume false
  (params (Key :type "Key Structure"))
  ;[1 1 1] Inputs
  (:`Pressed`
    (`self.InputQTE` 1)))

(event `Key|Z` :consume false
  (params (Key :type "Key Structure"))
  ;[1 1 1] Inputs
  (:`Pressed`
    (`self.InputQTE` 2)))

(event `EndGame`
  ;[1 1 1] Event END GAME
  (set `self.NeedPlayerAction` false)
  (`/Game/Blueprints/Ship.AddTimeGain` (`self.Ship`))
  (set `self.IsFinished` true)
  (set `self.IsPlaying` false)
  (`/Game/Blueprints/MG_Manager.IncrDecrCurrentGames` (`self.MGManager`) false true)
  (`self.LeaveGame`)
  (set `self.QteDone` 0))

(event `CreateQTE`
  (bind _returnvalue (`KismetMathLibrary.RandomFloatInRange` -50.0 50.0))
  (bind _numberofqte (`self.NumberOfQte`))
  (bind _returnvalue_2 (- (`self.NumberOfQte`) 1))
  (bind _output (`|GetArrayItem` (`self.QTERandom`) _returnvalue_2))
  (bind _output_2 (`|GetArrayItem` (`self.QTEFlipbooks`) _returnvalue_2))
  (bind _returnvalue_3 (- (* _returnvalue_2 (`self.xMultiplicator`)) 100.0))
  ;[1 1 1] CREATE QTE
  (if (not (== _numberofqte (`self.NumberOfInputs`)))
    (`/Engine/EditorBlueprintResources/StandardMacros.IncrementInt` _numberofqte
      (:`  `
        (bind _returnvalue_4 (`AddComponent|NODE_AddPaperFlipbookComponent-1`))
        (`KismetArrayLibrary.Array_Add` (`self.QTEFlipbooks`) _returnvalue_4)
        (`KismetArrayLibrary.Array_Add` (`self.QTERandom`) (`KismetMathLibrary.RandomInteger` 3))
        (if (== _output 0)
          (`SceneComponent.K2_SetRelativeLocation` _output_2 (`KismetMathLibrary.MakeVector` _returnvalue_3 11.0 _returnvalue) false false)
          (`SceneComponent.SetWorldScale3D` _output_2 (1.0 1.0 1.0))
          (`PaperFlipbookComponent.SetFlipbook` _output_2 "/Game/Anim/MiniGames/QTE_LeftClick.QTE_LeftClick")
          (elif (== _output 1)
            (`SceneComponent.K2_SetRelativeLocation` _output_2 (`KismetMathLibrary.MakeVector` _returnvalue_3 11.0 _returnvalue) false false)
            (`SceneComponent.SetWorldScale3D` _output_2 (1.5 1.5 1.5))
            (`PaperFlipbookComponent.SetFlipbook` _output_2 "/Game/Anim/MiniGames/QTE_Q.QTE_Q")
            (elif (== _output 2)
              (`SceneComponent.K2_SetRelativeLocation` _output_2 (`KismetMathLibrary.MakeVector` _returnvalue_3 11.0 _returnvalue) false false)
              (`SceneComponent.SetWorldScale3D` _output_2 (1.5 1.5 1.5))
              (`PaperFlipbookComponent.SetFlipbook` _output_2 "/Game/Anim/MiniGames/QTE_Z.QTE_Z"))))))))

(event `ClearQTE`
  (bind _qteflipbooks (`self.QTEFlipbooks`))
  ;[1 1 1] CLEAR QTE
  (`KismetArrayLibrary.Array_Clear` (`self.QTERandom`))
  (set `self.NumberOfQte` 0)
  (for _array_element _qteflipbooks
    (`ActorComponent.K2_DestroyComponent` _array_element))
  (`KismetArrayLibrary.Array_Clear` _qteflipbooks))

(fn `UserConstructionScript`)