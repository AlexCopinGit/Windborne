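; Manager actor that spawns a barrel-flight enemy once a randomized count of MGs is reached.
; BeginPlay caches the character, ship and MG manager, then rolls the threshold from a configured range.
; Tick compares the MG counter, which this graph never increments, to the threshold, then calls SpawnEnemy, resets and rerolls.
; SpawnEnemy spawns at the manager's location, guarded by IsSpawned, which is never cleared here.
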(event `self.ReceiveBeginPlay`
  (bind _mgsbeforeenemyvaluerange (`self.MGsBeforeEnemyValueRange`))
  (`|ExecutionSequence`
    (:`then_0`
      (bind _outactors (`GameplayStatics.GetAllActorsOfClass` "/Game/Blueprints/Char.Char_C"))
      (set `self.Char` (`|GetArrayItem` _outactors))
      (bind _outactors_2 (`GameplayStatics.GetAllActorsOfClass` "/Game/Blueprints/Ship.Ship_C"))
      (set `self.Ship` (`|GetArrayItem` _outactors_2))
      (bind _outactors_3 (`GameplayStatics.GetAllActorsOfClass` "/Game/Blueprints/MiniGames/MG_Manager.MG_Manager_C"))
      (set `self.MG_Manager` (`|GetArrayItem` _outactors_3)))
    (:`then_1`
      (set `self.MGsBeforeEnemyValue` (`KismetMathLibrary.RandomIntegerInRange` (`|GetArrayItem` _mgsbeforeenemyvaluerange) (`|GetArrayItem` _mgsbeforeenemyvaluerange 1))))))

(event `self.ReceiveTick`
  (params (DeltaSeconds :type "Float (single-precision)"))
  (bind _mgsbeforeenemyvaluerange (`self.MGsBeforeEnemyValueRange`))
  (set `self.DeltaTime` DeltaSeconds)
  (if (>= (`self.MGsBeforeEnemy`) (`self.MGsBeforeEnemyValue`))
    (`self.SpawnEnemy`)
    (set `self.MGsBeforeEnemy` 0)
    (set `self.MGsBeforeEnemyValue` (`KismetMathLibrary.RandomIntegerInRange` (`|GetArrayItem` _mgsbeforeenemyvaluerange) (`|GetArrayItem` _mgsbeforeenemyvaluerange 1)))))

(event `SpawnEnemy`
  (bind _returnvalue_location (`KismetMathLibrary.BreakTransform` (`self.GetTransform` self)))
  (if (not (`self.IsSpawned`))
    (bind _returnvalue (`|SpawnActorFromClass` "/Game/Blueprints/Enemy/Enemy_BarrelFlight_Blueprint.Enemy_BarrelFlight_Blueprint_C" (`KismetMathLibrary.MakeTransform` _returnvalue_location) "Undefined" "OverrideRootScale" null null))
    (set `self.EnemyBarrel` _returnvalue)
    (set `self.IsSpawned` true)))

(fn `UserConstructionScript`)