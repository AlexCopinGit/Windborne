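; Seagull enemy, a flipbook-animated character that plays a crash animation on spawn, climbs ladders and performs a timed attack.
; Tick checks overlapped ladders against floor numbers set by named overlap actors, gating the MoveUp axis climb, which switches to flying and a trigger collision profile.
; UpdateAnimation maps attack, climb and velocity state to flipbooks, several being Char-prefixed.
; Attacks require walking and freeze velocity for the current flipbook's length.
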(event `self.ReceiveBeginPlay`
  (bind _outactors (`GameplayStatics.GetAllActorsOfClass` "/Game/Blueprints/Char.Char_C"))
  (set `self.Char` (`|GetArrayItem` _outactors))
  (bind _outactors_2 (`GameplayStatics.GetAllActorsOfClass` "/Game/Blueprints/Ship.Ship_C"))
  (set `self.Ship` (`|GetArrayItem` _outactors_2))
  (set `self.JustSpawned` true))

(event `UpdateAnimation`
  (bind _returnvalue_x (`KismetMathLibrary.BreakVector` (`self.GetVelocity`)))
  (`|ExecutionSequence`
    (:`then_0`
      (if (`self.IsAttacking`)
        (set `self.AnimState` "NewEnumerator3")
        (elif (`self.IsMovingUp`)
          (set `self.AnimState` "NewEnumerator2")
          (elif (!= _returnvalue_x 0.0)
            (set `self.AnimState` "NewEnumerator1")
            (else
              (set `self.AnimState` "NewEnumerator0"))))))
    (:`then_1`
      (`PaperFlipbookComponent.SetFlipbook` (`self.Sprite`) (select `/Game/Blueprints/AnimState` (`self.AnimState`) :`NewEnumerator0` "/Game/Anim/Enemy/Enemy_Idle.Enemy_Idle" :`NewEnumerator1` "/Game/Anim/Enemy/Enemy_Walk.Enemy_Walk" :`NewEnumerator2` "/Game/Anim/Enemy/Enemy_Fall.Enemy_Fall" :`NewEnumerator3` "/Game/Anim/Char/CharAttack.CharAttack" :`NewEnumerator4` "/Game/Anim/Char/CharJumpStill.CharJumpStill" :`NewEnumerator5` "/Game/Anim/Char/CharJumpRun.CharJumpRun" :!type "PaperFlipbook Object Reference")))))

(event `InputAxis|MoveUp`
  (params (AxisValue :type "Float (single-precision)"))
  (bind _charactermovement (`self.CharacterMovement`))
  (bind _charactermovement_2 (`self.CharacterMovement`))
  (if (`self.CanClimb`)
    (if (and (`self.CanGoDown`) (< AxisValue 0.0))
      (set `self.IsMovingUp` true)
      (set `MovementComponent.Velocity` (`KismetMathLibrary.MakeVector` 0.0 0.0 (* -1 (`self.ClimbSpeed`))) _charactermovement)
      (`PrimitiveComponent.SetCollisionProfileName` (`self.CapsuleComponent`) "Trigger" true :!label _label)
      (`CharacterMovementComponent.SetMovementMode` _charactermovement_2 "MOVE_Flying" 0)
      (`KismetSystemLibrary.Delay` 0.18)
      (`GameplayStatics.PlaySound2D` (`self.SoundLadder01`) 0.5 1.0 0.0 null null)
      (`KismetSystemLibrary.Delay` 0.18)
      (`GameplayStatics.PlaySound2D` (`self.SoundLadder02`) 0.5 1.0 0.0 null null)
      (elif (and (`self.CanGoUp`) (> AxisValue 0.0))
        (set `self.IsMovingUp` true)
        (set `MovementComponent.Velocity` (`KismetMathLibrary.MakeVector` 0.0 0.0 (`self.ClimbSpeed`)) _charactermovement)
        (goto _label)
        (else
          (set `self.IsMovingUp` false :!label _label_2)
          (if (`CharacterMovementComponent.IsWalking` _charactermovement_2)
            (`CharacterMovementComponent.SetMovementMode` _charactermovement_2 "MOVE_Walking" 0)
            (else
              (`CharacterMovementComponent.SetMovementMode` _charactermovement_2 "MOVE_Falling" 0))))))
    (else
      (goto _label_2))))

(event `self.ReceiveTick`
  (params (DeltaSeconds :type "Float (single-precision)"))
  (bind _overlappingactors (`self.GetOverlappingActors` "/Game/Blueprints/Ladder.Ladder_C"))
  (`|ExecutionSequence`
    (:`then_1`
      (set `self.CanClimb` (`KismetArrayLibrary.Array_IsValidIndex` _overlappingactors))
      (bind _asladder (cast `/Game/Blueprints/Ladder` (`|GetArrayItem` _overlappingactors)))
      (set `self.CanGoDown` (== (`/Game/Blueprints/Ladder.CanGoDownOnFloor` _asladder) (`self.CurrentDownFloor`)))
      (set `self.CanGoUp` (== (`/Game/Blueprints/Ladder.CanGoUpOnFloor` _asladder) (`self.CurrentUpFloor`))))
    (:`then_2`
      (if (`self.IsAttacking`)
        (set `MovementComponent.Velocity` (0.0 0.0 0.0) (`self.CharacterMovement`))))
    (:`then_3`
      (if (`self.JustSpawned`)
        (`PaperFlipbookComponent.SetFlipbook` (`self.Sprite`) "/Game/Anim/Enemy/Enemy_Crash.Enemy_Crash")
        (`KismetSystemLibrary.Delay` (`PaperFlipbookComponent.GetFlipbookLength` (`self.Sprite`)))
        (`PaperFlipbookComponent.SetFlipbook` (`self.Sprite`) "/Game/Anim/Enemy/Enemy_Idle.Enemy_Idle")
        (`PrimitiveComponent.SetSimulatePhysics` (`self.CapsuleComponent`) false)
        (set `self.JustSpawned` false)))))

(event `self.ReceiveActorBeginOverlap`
  (params (OtherActor :type "Actor Object Reference"))
  (`|ExecutionSequence`
    (:`then_0`
      (switch `string` (`KismetSystemLibrary.GetObjectName` OtherActor)
        (:`DownFloor0`
          (set `self.CurrentDownFloor` 0))
        (:`DownFloor1`
          (set `self.CurrentDownFloor` 1))
        (:`DownFloor2`
          (set `self.CurrentDownFloor` 2)))
      (`PrimitiveComponent.SetCollisionProfileName` (`self.CapsuleComponent`) "Pawn" true))
    (:`then_1`
      (switch `string` (`KismetSystemLibrary.GetObjectName` OtherActor)
        (:`UpFloor0`
          (set `self.CurrentUpFloor` 0))
        (:`UpFloor1`
          (set `self.CurrentUpFloor` 1))
        (:`UpFloor2`
          (set `self.CurrentUpFloor` 2))))))

(event `EventAttack`
  (if (`CharacterMovementComponent.IsWalking` (`self.CharacterMovement`))
    (if (not (`self.IsAttacking`))
      (`GameplayStatics.PlaySound2D` "/Game/Sound/Swipe_Cue1.Swipe_Cue1" 0.5 1.0 0.0 null null)
      (set `self.IsAttacking` true)
      (`KismetSystemLibrary.Delay` (`PaperFlipbookComponent.GetFlipbookLength` (`self.Sprite`)))
      (set `self.IsAttacking` false))))

(fn `UserConstructionScript`)