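; Enemy barrel, a flipbook-based actor that flies horizontally toward the ship and then drops.
; BeginPlay picks a random destination X within a set range and records the starting X and Z.
; Tick keeps calling Play on a timeline that lerps X to the destination at constant height.
; When the timeline finishes, the barrel switches to its falling flipbook and enables gravity.
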(event `self.ReceiveBeginPlay`
  (bind (_returnvalue_x _returnvalue_y _returnvalue_z) (`KismetMathLibrary.BreakVector` (`self.K2_GetActorLocation`)))
  (bind _destinationxvaluerange (`self.DestinationXValueRange`))
  (set `self.DestinationX` (`KismetMathLibrary.RandomFloatInRange` (`|GetArrayItem` _destinationxvaluerange) (`|GetArrayItem` _destinationxvaluerange 1)))
  (set `self.OriginalX` _returnvalue_x)
  (set `self.OriginalZ` _returnvalue_z))

(event `self.ReceiveTick`
  (params (DeltaSeconds :type "Float (single-precision)"))
  (`self.MoveToTheShip`))

(event `MoveToTheShip`
  (bind (_direction _timex) (`Timeline|BarrelMovement`)
    (:`Update`
      (`self.K2_SetActorLocation` (`KismetMathLibrary.MakeVector` (`KismetMathLibrary.Lerp` (`self.OriginalX`) (`self.DestinationX`) _timex) 0.0 (`self.OriginalZ`))))
    (:`Finished`
      (`self.BarrelFall`))))

(event `BarrelFall`
  (`PaperFlipbookComponent.SetFlipbook` (`self.RenderComponent`) "/Game/Anim/Enemy/Barrel_Fall.Barrel_Fall")
  (`PrimitiveComponent.SetEnableGravity` (`self.RenderComponent`) true))

(fn `UserConstructionScript`)