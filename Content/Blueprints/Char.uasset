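; Paper2D side-scroller player character that runs left and right, with unfinished ladder climbing.
; Tick picks the sprite flipbook from an Idle/Run/Climb state and yaws the controller to face velocity, or the last input when stopped.
; Overlapping a Ladder enables up input, which zeroes gravity but sets location to the world origin.
; Climb has no flipbook, IsMovingUp is never set here, and the BeginPlay timeline's AltitudeValue is unused.
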(event `self.ReceiveBeginPlay`
  (`ActorComponent.SetIsReplicated` (`self.Sprite`) true)
  (bind (_direction _newtrack_0) (`Timeline|LoseAltitude`)
    (:`Update`
      (set `self.AltitudeValue` _newtrack_0))))

(event `InputAxis|MoveRight`
  (params (AxisValue :type "Float (single-precision)"))
  ;[1 1 1] Handle Movement
  (if (> AxisValue 0.0)
    (set `self.IsMovingRight` true)
    (elif (< AxisValue 0.0)
      (set `self.IsMovingRight` false)))
  (`self.AddMovementInput` (1.0 0.0 0.0) AxisValue))

(event `self.ReceiveTick`
  (params (DeltaSeconds :type "Float (single-precision)"))
  (bind _returnvalue (`self.GetController`))
  (bind _returnvalue_2 (`self.GetController`))
  ;[1 1 1] Tick - Updates animation
  (`|ExecutionSequence`
    (:`then_0`
      (`self.UpdateAnimation`)
      (`/Engine/EditorBlueprintResources/StandardMacros.CompareFloat` (.x (`MovementComponent.Velocity` (`self.GetMovementComponent`)))
        (:`>`
          (`/Engine/EditorBlueprintResources/StandardMacros.IsValid` _returnvalue_2 :!label _label
            (:`Is Valid`
              (`Controller.SetControlRotation` _returnvalue_2 (`KismetMathLibrary.MakeRotator` 0.0)))))
        (:`==`
          (if (`self.IsMovingRight`)
            (goto _label)
            (else
              (`/Engine/EditorBlueprintResources/StandardMacros.IsValid` _returnvalue :!label _label_2
                (:`Is Valid`
                  (`Controller.SetControlRotation` _returnvalue (`KismetMathLibrary.MakeRotator` 0.0 0.0 180.0)))))))
        (:`<`
          (goto _label_2))))
    (:`then_1`
      (set `self.CanClimb` (`KismetArrayLibrary.Array_IsValidIndex` (`self.GetOverlappingActors` "/Game/Blueprints/Ladder.Ladder_C"))))))

(event `InputAxis|MoveUp`
  (params (AxisValue :type "Float (single-precision)"))
  (if (`self.CanClimb`)
    (if (< AxisValue 0.0)
      _
      (elif (> AxisValue 0.0)
        (set `CharacterMovementComponent.GravityScale` 0.0 (`self.CharacterMovement`))
        (`self.K2_SetActorLocation` (0.0 0.0 0.0))))))

(event `UpdateAnimation`
  ;[1 1 1] Handle Animation
  (`|ExecutionSequence`
    (:`then_0`
      (if (> (`KismetMathLibrary.VSize` (`self.GetVelocity`)) 0.0)
        (if (`self.IsMovingUp`)
          (set `self.AnimState` "NewEnumerator2")
          (else
            (set `self.AnimState` "NewEnumerator1")))
        (else
          (set `self.AnimState` "NewEnumerator0"))))
    (:`then_1`
      (`PaperFlipbookComponent.SetFlipbook` (`self.Sprite`) (select `/Game/Blueprints/AnimState` (`self.AnimState`) :`NewEnumerator0` "/Game/Anim/Char/CharIdle.CharIdle" :`NewEnumerator1` "/Game/Anim/Char/CharRun.CharRun" :!type "PaperFlipbook Object Reference")))))

(fn `UserConstructionScript`)