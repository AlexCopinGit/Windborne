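; Ship actor that gains or loses altitude with the number of mini-games playing and houses a phonograph music player.
; Tick moves it vertically and updates a time-based altitude, falling faster with more active games and climbing when none run.
; Altitude percentage thresholds fire one-shot events that spawn a Step1 actor and despawn the character; other steps are empty.
; Attacking in the radio box cycles three fading tracks with a flipbook animation; keys adjust volume.
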(event `AddTimeGain`
  (set `self.AltitudeTimeGain` (+ (`self.AltitudeTimeGain`) (`self.AltitudeTimeGainValue`))))

(event `self.ReceiveBeginPlay`
  (bind _musicsarray (`self.MusicsArray`))
  (bind _output (`|GetArrayItem` _musicsarray))
  (`|ExecutionSequence`
    (:`then_0`
      (bind _outactors (`GameplayStatics.GetAllActorsOfClass` "/Game/Sprites/UI/MiniShip_Blueprint.MiniShip_Blueprint_C"))
      (set `self.MiniShip` (`|GetArrayItem` _outactors))
      (set `self.Altitude` (`self.TotalDuration`))
      (bind _outactors_2 (`GameplayStatics.GetAllActorsOfClass` "/Game/Blueprints/MG_Manager.MG_Manager_C"))
      (set `self.MGManager` (`|GetArrayItem` _outactors_2))
      (bind _outactors_3 (`GameplayStatics.GetAllActorsOfClass` "/Game/Blueprints/Char.Char_C"))
      (set `self.Char` (`|GetArrayItem` _outactors_3))
      (goto _label :!via `Reset`))
    (:`then_1`
      (`KismetArrayLibrary.Array_Add` (`self.MusicsArray`) (`self.Music01`))
      (`KismetArrayLibrary.Array_Add` (`self.MusicsArray`) (`self.Music02`))
      (`KismetArrayLibrary.Array_Add` _musicsarray (`self.Music03`))
      (`AudioComponent.FadeIn` _output 5.0 (`self.VolumeMultiplier`) 0.0 "Linear")
      (set `self.CurrentMusic` _output)
      (set `self.CurrentIndexMusic` 0))))

(event `Key|B`
  (params (Key :type "Key Structure"))
  ;[1 1 1] Lose or gain altitude
  (:`Pressed`
    (set `self.IsGainingAlt` true)))

(event `self.ReceiveTick`
  (params (DeltaSeconds :type "Float (single-precision)"))
  (bind _altitude (`self.Altitude`))
  (bind _deltatime (`self.DeltaTime`))
  (bind _totalduration (`self.TotalDuration`))
  (bind (_returnvalue_x _returnvalue_y _returnvalue_z) (`KismetMathLibrary.BreakVector` (`self.K2_GetActorLocation` self)))
  (bind _returnvalue (* (`self.NumberOfGamesPlaying`) (* (`self.AltitudeLoss`) (`self.AtitudeLossMultiplicator`))))
  (set `self.DeltaTime` DeltaSeconds)
  (`|ExecutionSequence`
    (:`then_0`
      ;[1 1 1] Lose or gain altitude
      (if (`self.IsGainingAlt`)
        (`self.K2_SetActorLocation` (`KismetMathLibrary.MakeVector` 0.0 0.0 (+ _returnvalue_z _returnvalue)))
        (else
          (`self.K2_SetActorLocation` (`KismetMathLibrary.MakeVector` 0.0 0.0 (- _returnvalue_z _returnvalue)))))
      (set `self.AltitudePercentage` (/ (`KismetMathLibrary.FClamp` (`self.Altitude`) 0.0 _totalduration) _totalduration)))
    (:`then_2`
      (`self.EventsAltitudeSteps`)
      (if (`self.IsGainingAlt`)
        (set `self.Altitude` (`KismetMathLibrary.FClamp` (+ _altitude _deltatime) 0.0 (`self.TotalDuration`)))
        (else
          (set `self.Altitude` (- _altitude (* (`self.NumberOfGamesPlaying`) _deltatime))))))
    (:`then_3`
      (if (> (`self.NumberOfGamesPlaying`) 0)
        (set `self.IsGainingAlt` false)
        (else
          (set `self.IsGainingAlt` true))))))

(event `Key|Add` :consume false
  (params (Key :type "Key Structure"))
  (:`Pressed`
    (bind _output_get (set `self.VolumeMultiplier` (`KismetMathLibrary.FClamp` (+ (`self.VolumeMultiplier`) 0.1) 0.1)))
    (`AudioComponent.SetVolumeMultiplier` (`self.CurrentMusic`) _output_get)
    (`KismetSystemLibrary.PrintString` (`KismetStringLibrary.Conv_DoubleToString` _output_get))))

(event `Key|Subtract` :consume false
  (params (Key :type "Key Structure"))
  (:`Pressed`
    (bind _output_get (set `self.VolumeMultiplier` (`KismetMathLibrary.FClamp` (- (`self.VolumeMultiplier`) 0.1) 0.1)))
    (`AudioComponent.SetVolumeMultiplier` (`self.CurrentMusic`) _output_get)
    (`KismetSystemLibrary.PrintString` (`KismetStringLibrary.Conv_DoubleToString` _output_get))))

(event `EventsAltitudeSteps`
  (bind _altitudesteps (`self.AltitudeSteps`))
  (bind _altitudepercentage (`self.AltitudePercentage`))
  ;[1 1 1] Events Steps
  (`|ExecutionSequence`
    (:`then_0`
      (if (< _altitudepercentage (`|GetArrayItem` _altitudesteps))
        (`/Engine/EditorBlueprintResources/StandardMacros.DoOnce` false)))
    (:`then_1`
      (if (< _altitudepercentage (`|GetArrayItem` _altitudesteps 1))
        _))
    (:`then_2`
      (if (< _altitudepercentage (`|GetArrayItem` _altitudesteps 2))
        (`/Engine/EditorBlueprintResources/StandardMacros.DoOnce` false)))
    (:`then_3`
      (if (< _altitudepercentage (`|GetArrayItem` _altitudesteps 3))
        (`/Engine/EditorBlueprintResources/StandardMacros.DoOnce` false
          (:`Completed`
            (bind _returnvalue (`|SpawnActorFromClass` (`self.Step1`) (`KismetMathLibrary.MakeTransform` (`KismetMathLibrary.MakeVector` 0.0 -2.0 (- (.z (.location (`self.GetTransform` self))) 400.0)) (`KismetMathLibrary.MakeRotator` 90.0)) "AlwaysSpawn" "OverrideRootScale" self null))
            (set `self.Step1Actor` _returnvalue)))))
    (:`then_4`
      (if (<= (`self.AltitudePercentage`) (`|GetArrayItem` _altitudesteps 4))
        (`/Engine/EditorBlueprintResources/StandardMacros.DoOnce` false :!label _label
          (:`Completed`
            (`/Game/Blueprints/Char.Dispawn` (`self.Char`))))))))

(event `InputAction|Attack` :consume false
  (params (Key :type "Key Structure"))
  (:`Pressed`
    (if (`PrimitiveComponent.IsOverlappingActor` (`self.BoxRadio`) (`self.Char`))
      (`self.ChangeMusic`))))

(event `ChangeMusic`
  (bind _phonographe (`self.Phonographe`))
  (bind _volumemultiplier (`self.VolumeMultiplier`))
  (bind _output (`|GetArrayItem` (`self.MusicsArray`) (`self.CurrentIndexMusic`)))
  (`PaperFlipbookComponent.SetFlipbook` (`self.Phonographe`) "/Game/Anim/Ship/Phonographe_Hit.Phonographe_Hit")
  (`AudioComponent.FadeOut` (`|GetArrayItem` (`self.MusicsArray`) (`self.CurrentIndexMusic`)) 0.5 0.0 "Linear")
  (set `self.CurrentMusic` null)
  (if (== (`self.CurrentIndexMusic`) (- (`KismetArrayLibrary.Array_Length` (`self.MusicsArray`)) 1))
    (set `self.CurrentIndexMusic` 0)
    (`AudioComponent.FadeIn` _output 2.0 _volumemultiplier 0.0 "Linear")
    (set `self.CurrentMusic` _output)
    (else
      (`/Engine/EditorBlueprintResources/StandardMacros.IncrementInt` (`self.CurrentIndexMusic`)
        (:`  `
          (`AudioComponent.FadeIn` _output 2.0 _volumemultiplier 0.0 "Linear")
          (set `self.CurrentMusic` _output)))))
  (`KismetSystemLibrary.Delay` (`PaperFlipbookComponent.GetFlipbookLength` _phonographe))
  (`PaperFlipbookComponent.SetFlipbook` _phonographe "/Game/Anim/Ship/Phonographe_Idle.Phonographe_Idle"))

(fn `UserConstructionScript`)