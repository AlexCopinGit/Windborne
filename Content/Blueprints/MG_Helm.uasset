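; MG_Helm is a helm minigame station on the ship that the player can join when it needs action.
; Tick swaps idle and warning flipbooks; character overlap enables interaction, which toggles a blur widget, camera focus, HUD and player input.
; Win clears the request, adds ship time gain, updates the minigame manager's count and exits.
; GameplayLoop is an empty stub, and a debug J key triggers the request.
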(event `Key|J` :consume false
  (params (Key :type "Key Structure"))
  ;[1 1 1] Debug
  (:`Pressed`
    (set `self.NeedPlayerAction` true)))

(event `self.ReceiveActorBeginOverlap`
  (params (OtherActor :type "Actor Object Reference"))
  (cast `/Game/Blueprints/Char` OtherActor)
  (if (`self.NeedPlayerAction`)
    (set `self.CanPlayerInteract` true)
    (`PaperFlipbookComponent.SetFlipbook` (`self.PaperFlipbook`) "/Game/Anim/MiniGames/MG_Helm_Interact.MG_Helm_Interact")))

(event `self.ReceiveActorEndOverlap`
  (params (OtherActor :type "Actor Object Reference"))
  (cast `/Game/Blueprints/Char` OtherActor)
  (set `self.CanPlayerInteract` false))

(event `InputAction|Interact`
  (params (Key :type "Key Structure"))
  (:`Pressed`
    (if (`self.IsActive`)
      (`self.Leave`)
      (elif (and (`self.NeedPlayerAction`) (`self.CanPlayerInteract`))
        (`self.Join`)))))

(event `self.ReceiveBeginPlay`
  (bind _returnvalue (`|CreateWidget` "/Game/UI/MG_Blur.MG_Blur_C"))
  (bind _output_get (set `self.Widget` _returnvalue))
  (`UserWidget.AddToViewport` _output_get 0)
  (`Widget.SetVisibility` _output_get "Hidden")
  (bind _outactors (`GameplayStatics.GetAllActorsOfClass` "/Game/Blueprints/Ship.Ship_C"))
  (set `self.Ship` (`|GetArrayItem` _outactors))
  (bind _outactors_2 (`GameplayStatics.GetAllActorsOfClass` "/Game/Blueprints/Char.Char_C"))
  (set `self.Player` (`|GetArrayItem` _outactors_2))
  (bind _outactors_3 (`GameplayStatics.GetAllActorsOfClass` "/Game/Blueprints/MG_Manager.MG_Manager_C"))
  (set `self.MGManager` (`|GetArrayItem` _outactors_3))
  (set `self.LocOffset` (`self.K2_GetActorLocation`)))

(event `self.ReceiveTick`
  (params (DeltaSeconds :type "Float (single-precision)"))
  (bind _paperflipbook (`self.PaperFlipbook`))
  (`|ExecutionSequence`
    (:`then_0`
      (if (`self.NeedPlayerAction`)
        (set `self.IsPlaying` true)
        (if (not (`self.CanPlayerInteract`))
          (`PaperFlipbookComponent.SetFlipbook` _paperflipbook "/Game/Anim/MiniGames/MG_Helm_Warning.MG_Helm_Warning"))
        (else
          (`PaperFlipbookComponent.SetFlipbook` _paperflipbook "/Game/Anim/MiniGames/MG_Helm_Idle.MG_Helm_Idle"))))
    (:`then_1`
      (`self.GameplayLoop`))))

(event `Join`
  (`Widget.SetVisibility` (`self.Widget`) "Visible")
  (`/Game/Blueprints/Cam.FocusMG` (`/Game/Blueprints/MG_Manager.MainCam` (`self.MGManager`)) true (`self.LocOffset`))
  (`/Game/UI/HUD_Main.ShowWidgets` (`/Game/Blueprints/MG_Manager.HUD` (`self.MGManager`)) false)
  (`self.DisableInput` (`self.Player`) null)
  (set `self.IsActive` true))

(event `Leave`
  (`Widget.SetVisibility` (`self.Widget`) "Hidden")
  (`/Game/Blueprints/Cam.FocusMG` (`/Game/Blueprints/MG_Manager.MainCam` (`self.MGManager`)) false (0.0 0.0 0.0))
  (`self.EnableInput` (`self.Player`) null)
  (set `self.IsActive` false))

(event `Win`
  (set `self.NeedPlayerAction` false)
  (set `self.IsFinished` true)
  (set `self.IsPlaying` false)
  (`/Game/Blueprints/Ship.AddTimeGain` (`self.Ship`))
  (`/Game/Blueprints/MG_Manager.IncrDecrCurrentGames` (`self.MGManager`) false true)
  (`self.Leave`))

(event `GameplayLoop`)

(fn `UserConstructionScript`)