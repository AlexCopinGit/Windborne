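; AudioMenu is an actor Blueprint that lets the player adjust the volume of its Audio component, apparently menu audio, from the keyboard.
; The Add and Subtract keys step VolumeMultMenu up or down by a fixed amount, clamped so it never reaches silence, then apply it as the component's volume multiplier.
; BeginPlay, overlap, Tick and the construction script contain no logic.
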(event `Key|Add` :consume false
  (params (Key :type "Key Structure"))
  (:`Pressed`
    (bind _output_get (set `self.VolumeMultMenu` (`KismetMathLibrary.FClamp` (+ (`self.VolumeMultMenu`) 0.1) 0.1)))
    (`AudioComponent.SetVolumeMultiplier` (`self.Audio`) _output_get)))

(event `Key|Subtract` :consume false
  (params (Key :type "Key Structure"))
  (:`Pressed`
    (bind _output_get (set `self.VolumeMultMenu` (`KismetMathLibrary.FClamp` (- (`self.VolumeMultMenu`) 0.1) 0.1)))
    (`AudioComponent.SetVolumeMultiplier` (`self.Audio`) _output_get)))

(event `self.ReceiveBeginPlay`)

(fn `UserConstructionScript`)