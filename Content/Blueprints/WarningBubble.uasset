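; WarningBubble is a flipbook sprite actor that serves as a bobbing warning indicator, shown as soon as it spawns.
; Tick lerps the sprite's alpha toward a target set by the IsVisible flag and adds a small cosine-driven vertical offset.
; Appear shows the flipbook and sets the flag.
; Disappear clears the flag but destroys the actor immediately, so no fade-out plays.
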(event `self.ReceiveTick`
  (params (DeltaSeconds :type "Float (single-precision)"))
  (bind _paperflipbook (`self.PaperFlipbook`))
  (bind (_spritecolor_r _spritecolor_g _spritecolor_b) (break `LinearColor` (`PaperFlipbookComponent.SpriteColor` _paperflipbook)))
  (`|ExecutionSequence`
    (:`then_0`
      (if (`self.IsVisible`)
        (set `self.FinalAlpha` 255.0)
        (else
          (set `self.FinalAlpha` 0.0)))
      (bind _output_get (set `self.CurrentAlpha` (`KismetMathLibrary.Lerp` (`self.CurrentAlpha`) (`self.FinalAlpha`) DeltaSeconds)))
      (`PaperFlipbookComponent.SetSpriteColor` _paperflipbook (make `LinearColor` _spritecolor_r _spritecolor_g _spritecolor_b _output_get)))
    (:`then_1`
      (`self.K2_AddActorLocalOffset` (`KismetMathLibrary.MakeVector` 0.0 0.0 (/ (`KismetMathLibrary.Cos` (`self.GetGameTimeSinceCreation`)) 20.0))))))

(event `self.ReceiveBeginPlay`
  (`self.Appear`))

(event `Appear`
  (`SceneComponent.SetVisibility` (`self.PaperFlipbook`) true false)
  (set `self.IsVisible` true))

(event `Disappear`
  (set `self.IsVisible` false)
  (`SceneComponent.SetVisibility` (`self.PaperFlipbook`) true false)
  (`self.K2_DestroyActor`))

(fn `UserConstructionScript`)