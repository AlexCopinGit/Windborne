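; Paper2D explosive minigame actor where the player mashes C to fill a bar and make the Ship gain altitude.
; While HasBegun is set, it plays the TNT flipbook, and an overlapping Char enables input and reveals the MG_SpamBar widget.
; Each press adds clamped progress, while Tick constantly drains it.
; A full bar marks the win, ends the game, hides the widget and sets IsGainingAlt on the first Ship found.
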(event `self.ReceiveBeginPlay`
  (bind _returnvalue (`|CreateWidget` "/Game/UI/MG_SpamBar.MG_SpamBar_C"))
  (bind _output_get (set `self.SpamBar` _returnvalue))
  (`UserWidget.AddToViewport` _output_get 0)
  (`Widget.SetVisibility` _output_get "Hidden"))

(event `self.ReceiveTick`
  (params (DeltaSeconds :type "Float (single-precision)"))
  (`|ExecutionSequence`
    (:`then_0`
      (`self.SpamGameEvent` DeltaSeconds))
    (:`then_1`
      (set `self.SpamCurrentValuePerc` (- (`self.SpamCurrentValuePerc`) DeltaSeconds)))))

(event `SpamGameEvent`
  (params (DeltaTime :type "Float (double-precision)"))
  (bind _paperflipbook (`self.PaperFlipbook`))
  (bind _returnvalue (`KismetMathLibrary.NearlyEqual_FloatFloat` (`self.SpamCurrentValuePerc`) 1.0))
  ;[1 1 1] EventSpamGame
  (if (`self.HasBegun`)
    (`PaperFlipbookComponent.SetFlipbook` _paperflipbook "/Game/Anim/MiniGame/MiniGameTNT.MiniGameTNT")
    (if (`self.HasWon`)
      _
      (elif _returnvalue
        (set `self.HasWon` _returnvalue)
        (set `self.HasBegun` false)
        (bind _outactors (`GameplayStatics.GetAllActorsOfClass` "/Game/Blueprints/Ship.Ship_C"))
        (set `/Game/Blueprints/Ship.IsGainingAlt` true (`|GetArrayItem` _outactors))
        (`Widget.SetVisibility` (`self.SpamBar`) "Hidden")))
    (else
      (`PaperFlipbookComponent.SetFlipbook` _paperflipbook "/Game/Anim/MiniGame/MG_Explosive_Idle.MG_Explosive_Idle"))))

(event `Key|C`
  (params (Key :type "Key Structure"))
  (bind _spamcurrentvalueperc (`self.SpamCurrentValuePerc`))
  ;[1 1 1] Input Space
  (:`Pressed`
    (if (`self.HasBegun`)
      (if (`self.IsInRange`)
        (set `self.SpamCurrentValuePerc` (`KismetMathLibrary.FClamp` (+ (/ (`self.SpamValue`) (`self.SpamTotalValue`)) _spamcurrentvalueperc)))
        (`KismetSystemLibrary.PrintString` (`KismetStringLibrary.Conv_DoubleToString` _spamcurrentvalueperc))))))

(event `self.ReceiveActorBeginOverlap`
  (params (OtherActor :type "Actor Object Reference"))
  ;[1 1 1] Collision
  (if (`self.HasBegun`)
    (cast `/Game/Blueprints/Char` OtherActor)
    (set `self.IsInRange` true)
    (`Widget.SetVisibility` (`self.SpamBar`) "Visible")))

(event `self.ReceiveActorEndOverlap`
  (params (OtherActor :type "Actor Object Reference"))
  ;[1 1 1] Collision
  (cast `/Game/Blueprints/Char` OtherActor)
  (set `self.IsInRange` false)
  (`Widget.SetVisibility` (`self.SpamBar`) "Hidden"))

(fn `UserConstructionScript`)