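; AltBar is an altitude gauge that shows the Ship's altitude by moving an Indicator component vertically.
; On BeginPlay it finds all Ship actors and caches the first one.
; Each Tick it scales the Ship's AltitudePercentage by a fixed travel distance and applies the result as the Indicator's relative Z.
; The current Z is also stored each frame but is not used in the movement, which has no smoothing.
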(event `self.ReceiveBeginPlay`
  (bind _outactors (`GameplayStatics.GetAllActorsOfClass` "/Game/Blueprints/Ship.Ship_C"))
  (set `self.Ship` (`|GetArrayItem` _outactors)))

(event `self.ReceiveTick`
  (params (DeltaSeconds :type "Float (single-precision)"))
  (bind _indicator (`self.Indicator`))
  (bind (_relativelocation_x _relativelocation_y _relativelocation_z) (`KismetMathLibrary.BreakVector` (`SceneComponent.RelativeLocation` _indicator)))
  (`|ExecutionSequence`
    (:`then_0`
      (set `self.CurrentZ` _relativelocation_z)
      (set `self.NewZ` (* (`/Game/Blueprints/Ship.AltitudePercentage` (`self.Ship`)) 215.0)))
    (:`then_1`
      (`SceneComponent.K2_SetRelativeLocation` _indicator (`KismetMathLibrary.MakeVector` 0.0 0.0 (`self.NewZ`)) false false))))

(fn `UserConstructionScript`)