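; Camera actor that becomes the player's view and follows the first Ship in the level in a side-on plane.
; Each tick it lerps toward the ship plus its starting location as offset, shifted along X by player pawn velocity for look-ahead.
; It requests an idle camera shake every tick, then snaps X and Z to a pixel grid and pins Y to zero.
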(event `self.ReceiveBeginPlay`
  (`|ExecutionSequence`
    (:`then_0`
      (`PlayerController.SetViewTargetWithBlend` (`GameplayStatics.GetPlayerController` 0) self 0.0 "VTBlend_Linear" 0.0 false))
    (:`then_1`
      (set `self.LocOffset` (`self.K2_GetActorLocation`)))
    (:`then_2`
      (bind _outactors (`GameplayStatics.GetAllActorsOfClass` "/Game/Blueprints/Ship.Ship_C"))
      (bind _output_get (set `self.Boat` (`|GetArrayItem` _outactors)))
      (set `self.Target` _output_get))))

(event `self.ReceiveTick`
  (params (DeltaSeconds :type "Float (single-precision)"))
  (bind (_returnvalue_x _returnvalue_y _returnvalue_z) (`KismetMathLibrary.BreakVector` (`self.K2_GetActorLocation`)))
  (bind _pixelgridsize (`self.PixelGridSize`))
  (bind _returnvalue_x_2 (`KismetMathLibrary.BreakVector` (`self.GetVelocity` (`GameplayStatics.GetPlayerPawn` 0))))
  (`|ExecutionSequence`
    (:`then_0`
      (`self.K2_SetActorLocation` (`KismetMathLibrary.VLerp` (`self.K2_GetActorLocation`) (+ (+ (`self.K2_GetActorLocation` (`self.Target`)) (`self.LocOffset`)) (`KismetMathLibrary.MakeVector` (/ _returnvalue_x_2 (`self.PlayerVelocityFactor`)))) DeltaSeconds))
      (`PlayerController.ClientPlayCameraShakeFromSource` (`GameplayStatics.GetPlayerController` 0) "/Game/Blueprints/CamShake_Idle.CamShake_Idle_C" null))
    (:`then_1`
      (`self.K2_SetActorLocation` (`KismetMathLibrary.MakeVector` (`KismetMathLibrary.GridSnap_Float` _returnvalue_x _pixelgridsize) 0.0 (`KismetMathLibrary.GridSnap_Float` _returnvalue_z _pixelgridsize))))))

(fn `UserConstructionScript`)