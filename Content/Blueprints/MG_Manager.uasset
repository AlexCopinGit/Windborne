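; MG_Manager is a manager Blueprint that gathers references to core gameplay objects when play begins.
; On BeginPlay it stores the first Char actor as Character and the first Cam actor as MainCam through actor searches.
; It also casts the first player controller's HUD to HUD_Main and keeps it in HUD.
; No other logic is implemented, as Tick, overlap and the construction script are empty.
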(event `self.ReceiveBeginPlay`
  (`|ExecutionSequence`
    (:`then_0`
      (bind _outactors (`GameplayStatics.GetAllActorsOfClass` "/Game/Blueprints/Char.Char_C"))
      (set `self.Character` (`|GetArrayItem` _outactors))
      (bind _outactors_2 (`GameplayStatics.GetAllActorsOfClass` "/Game/Blueprints/Cam.Cam_C"))
      (set `self.MainCam` (`|GetArrayItem` _outactors_2))
      (bind _ashud_main (cast `/Game/UI/HUD_Main` (`PlayerController.GetHUD` (`GameplayStatics.GetPlayerController` 0))))
      (set `self.HUD` _ashud_main))))

(fn `UserConstructionScript`)